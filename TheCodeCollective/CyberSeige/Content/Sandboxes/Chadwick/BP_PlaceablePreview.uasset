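; Placeable preview Blueprint that detects whether other actors overlap its Box component.
; Each Tick it calls CheckForObstructions, which returns true when the Box has at least one overlapping actor and the first is valid.
; The Tick event discards that result, so the check currently drives no visible change or state.
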(event `self.ReceiveTick`
  (params (DeltaSeconds :type "Float (single-precision)"))
  (`self.CheckForObstructions`))

(fn `CheckForObstructions`
  (returns (Obstructed :type Boolean))
  (bind _overlappingactors (`PrimitiveComponent.GetOverlappingActors` (`self.Box`) null))
  (if (> (`KismetArrayLibrary.Array_Length` _overlappingactors) 0)
    (if (`KismetSystemLibrary.IsValid` (`|GetArrayItem` _overlappingactors))
      (return true)
      (else
        _)))
  (return false))

(fn `UserConstructionScript`)