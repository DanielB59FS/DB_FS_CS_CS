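; Shop display actor that animates five weapon preview components (pistol, assault rifle, LMG, sniper and rocket launcher) with a hover and spin.
; Tick advances a hover phase and a yaw angle by their speed variables, resetting each to zero after a full cycle.
; The bob adds a cosine-scaled world Z offset every frame, so its travel depends on frame rate, while the spin sets absolute world yaw on all five.
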(event `self.ReceiveTick`
  (params (DeltaSeconds :type "Float (single-precision)"))
  (set `self.WeaponHoverRads` (+ (* DeltaSeconds (`self.HoverSpeed`)) (`self.WeaponHoverRads`)))
  (set `self.WeaponRotateDegrees` (+ (* DeltaSeconds (`self.RotateSpeed`)) (`self.WeaponRotateDegrees`)))
  (if (> (`self.WeaponHoverRads`) 6.28)
    (set `self.WeaponHoverRads` 0.0))
  (if (> (`self.WeaponRotateDegrees`) 360.0)
    (set `self.WeaponRotateDegrees` 0.0))
  (`self.Apply Hover Offset` (`self.WeaponHoverRads`))
  (`self.Apply Rotate Offset` (`self.WeaponRotateDegrees`)))

(event `Apply Hover Offset`
  (params (Offset :type "Float (double-precision)"))
  (bind _returnvalue (`KismetMathLibrary.MakeVector` 0.0 0.0 (* (`KismetMathLibrary.Cos` Offset) 0.25)))
  (`SceneComponent.K2_AddWorldOffset` (`self.Pistol`) _returnvalue false false)
  (`SceneComponent.K2_AddWorldOffset` (`self.AssaultRifle`) _returnvalue false false)
  (`SceneComponent.K2_AddWorldOffset` (`self.LMG`) _returnvalue false false)
  (`SceneComponent.K2_AddWorldOffset` (`self.Sniper`) _returnvalue false false)
  (`SceneComponent.K2_AddWorldOffset` (`self.RocketLauncher`) _returnvalue false false))

(event `Apply Rotate Offset`
  (params (Offset :type "Float (double-precision)"))
  (bind _returnvalue (`KismetMathLibrary.MakeRotator` 0.0 0.0 Offset))
  (`SceneComponent.K2_SetWorldRotation` (`self.Pistol`) _returnvalue false false)
  (`SceneComponent.K2_SetWorldRotation` (`self.AssaultRifle`) _returnvalue false false)
  (`SceneComponent.K2_SetWorldRotation` (`self.LMG`) _returnvalue false false)
  (`SceneComponent.K2_SetWorldRotation` (`self.Sniper`) _returnvalue false false)
  (`SceneComponent.K2_SetWorldRotation` (`self.RocketLauncher`) _returnvalue false false))

(fn `UserConstructionScript`)