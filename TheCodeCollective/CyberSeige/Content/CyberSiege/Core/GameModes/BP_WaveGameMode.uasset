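; Wave survival game mode that alternates a skippable fortify countdown with defense phases until the final wave is won.
; While the timer is toggled on, Tick drives the Delay-based countdown shown on the player HUD, then hands the wave number to BP_WaveManager.
; Enemy added and died events track the count, ending the wave and the GameInstance time streak at zero.
; Older tag-based spawner logic remains but is disconnected.
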(event `Toggle Timer`
  (set `self.bStartTimer` (not (`self.bStartTimer`))))

(event `self.ReceiveBeginPlay`
  (bind _asbp_base_player (cast `/Game/CyberSiege/Core/Actors/Characters/BP_BasePlayer` (`GameplayStatics.GetPlayerPawn` 0))
    (:`then`
      (add `/Game/CyberSiege/Core/Actors/Characters/BP_BasePlayer.SkipFortifyPhase` _asbp_base_player (`|CreateDelegate` :!event `SkipFortifyPhase`))
      (bind _outactors (`GameplayStatics.GetAllActorsOfClass` "/Game/CyberSiege/Core/Engine/BP_WaveManager.BP_WaveManager_C"))
      (for _array_element _outactors
        (if (`KismetSystemLibrary.IsValid` _array_element)
          (set `self.WaveManager` _array_element))))
    (:`CastFailed`
      (`KismetSystemLibrary.PrintString` "Player is not BP_BasePlayer (WaveGameMode)"))))

(event `self.ReceiveTick`
  (params (DeltaSeconds :type "Float (single-precision)"))
  (if (`self.bStartTimer`)
    (if (not (`self.DefensePhase`))
      (`self.FortifyPhase`))))

(event `Enemy Added`
  (`/Engine/EditorBlueprintResources/StandardMacros.IncrementInt` (`self.Enemy Count`)
    (:`  `
      (`self.OnEnemyCount`))))

(event `Enemy Died`
  (`/Engine/EditorBlueprintResources/StandardMacros.DecrementInt` (`self.Enemy Count`)
    (:`  `
      (`self.OnEnemyCount`)
      (`self.Check Enemy Count`))))

(event `Check Enemy Count`
  (if (<= (`self.Enemy Count`) 0)
    (`/Game/CyberSiege/Core/Engine/BP_GameInstance.TimeStreakEnd` (cast `/Game/CyberSiege/Core/Engine/BP_GameInstance` (`GameplayStatics.GetGameInstance`) :!pure true))
    (`/Game/CyberSiege/Core/Interfaces/BPI_Enemies.AllEnemiesDead`)
    (set `self.DefensePhase` false)
    (`WaveManager.OnWaveEnded` (`self.WaveManager`))
    (if (== (`self.WaveCount`) (`WaveManager.FinalWave` (`self.WaveManager`)))
      (`self.GameEnded` "You Win!"))))

(event `FortifyPhase`
  (if (!= (`self.CountDownToDefensePhase`) 0)
    (if (== (`self.Count Down Timer`) null)
      (`self.SetCountdownTimer`))
    (if (>= (`self.CountDownToDefensePhase`) (`self.ResetCountdown`))
      (`/Engine/EditorBlueprintResources/StandardMacros.DoOnce` false :!label _label
        (:`Completed`
          (`Widget.SetVisibility` (`self.Count Down Timer`) "Visible")
          (`self.OnRoundEnded`))))
    (`KismetSystemLibrary.Delay` 1.0)
    (set `self.CountDownToDefensePhase` (- (`self.CountDownToDefensePhase`) 1))
    (`self.FortifyPhase`)
    (else
      (set `self.DefensePhase` true)
      (set `self.CountDownToDefensePhase` (`self.ResetCountdown`))
      (set `self.WaveCount` (+ (`self.WaveCount`) 1))
      (`Widget.SetVisibility` (`self.Count Down Timer`) "Hidden")
      (set `self.SpawnerLoopVariable` 0)
      (set `self.IndividualLoopVariable` 1)
      (`self.Spawners`)
      (goto _label :!via `Reset`))))

(event `Spawners`
  (bind _wavemanager (`self.WaveManager`))
  (bind _wavecount (`self.WaveCount`))
  (bind _asbp_game_instance (cast `/Game/CyberSiege/Core/Engine/BP_GameInstance` (`GameplayStatics.GetGameInstance`) :!pure true))
  (if (`KismetSystemLibrary.IsValid` (`self.WaveManager`))
    (`WaveManager.StartWaveProcess` _wavemanager _wavecount)
    (`/Game/CyberSiege/Core/Widgets/WBP_HUD.SetWave` (cast `/Game/CyberSiege/Core/Widgets/WBP_HUD` (`HUDManager.GetGameplayHUD` (cast `HUDManager` (`PlayerController.GetHUD` (`GameplayStatics.GetPlayerController` 0)) :!pure true)) :!pure true) _wavecount)
    (`/Game/CyberSiege/Core/Engine/BP_GameInstance.SetTimedThreshold` _asbp_game_instance (`WaveManager.SpawnList` _wavemanager))
    (`/Game/CyberSiege/Core/Engine/BP_GameInstance.TimeStreakStart` _asbp_game_instance)))

(event `SkipFortifyPhase`
  (if (and (not (`self.DefensePhase`)) (`self.bStartTimer`))
    (`Widget.SetVisibility` (`self.Count Down Timer`) "Hidden")
    (set `self.CountDownToDefensePhase` 1)))

(fn `Cast To Correct Spawner`
  (params (SpawnerLoopVariable :type Integer) (Spawner :type "Actor Object Reference"))
  (bind _returnvalue (`GameplayStatics.GetObjectClass` Spawner))
  (bind _returnvalue_2 (`GameplayStatics.GetObjectClass` Spawner))
  (if (and (== (mod (`self.WaveCount`) 2) 1) (or (== _returnvalue_2 null) (== _returnvalue_2 null) (== _returnvalue_2 null) (== _returnvalue_2 null) (== _returnvalue_2 null)))
    (message `/Game/CyberSiege/Core/Interfaces/BPI_Enemies.CallSpawners` Spawner null :!label _label)
    (elif (and (== (mod (`self.WaveCount`) 2) 0) (or (== _returnvalue null) (== _returnvalue null) (== _returnvalue null)))
      (goto _label)
      (else
        _)))
  (return))

(fn `Get Wave Manager`
  (returns (`Wave Manager` :type "/Game/CyberSiege/Core/Engine/BP_WaveManager Object Reference")))

(fn `GetEnemyCount`
  (returns (EnemyCount :type Integer))
  (return 0))

(fn `GetLHSLocation`
  (returns (LeftHandSocket :type "Vector Structure"))
  (return (0.0 0.0 0.0)))

(fn `IsEnemy`
  (returns (Boolean :type Boolean))
  (return false))

(fn `SetCountdownTimer`
  ;[1 1 1] Needs fixing, this completely break encapsultion
  (bind _asbp_base_player (cast `/Game/CyberSiege/Core/Actors/Characters/BP_BasePlayer` (`GameplayStatics.GetPlayerPawn` 0)))
  (set `self.Count Down Timer` (`/Game/CyberSiege/Core/Widgets/WBP_HUD.CountDownTimer` (`/Game/CyberSiege/Core/Actors/Characters/BP_BasePlayer.Get Gameplay HUD` _asbp_base_player))))

(fn `UserConstructionScript`)