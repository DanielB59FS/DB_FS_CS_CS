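; BP_WeaponDispenser is an interactable actor that gives the player a weapon of its configured class.
; When a targeting BP_BasePlayer interacts, it spawns WeaponClass at a far-off placeholder location.
; It then passes the new weapon to the player's WeaponHolster to replace a weapon, has the player equip it, and completes a quest step through BPQuestTriggerComponent.
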(event `/Game/CyberSiege/Core/Interfaces/BPI_Interact.Interact`
  (params (`Interacting Actor` :type "Actor Object Reference"))
  (bind _asbp_base_player (cast `/Game/CyberSiege/Core/Actors/Characters/BP_BasePlayer` `Interacting Actor`))
  (if (and (`self.bTargetedByPlayer`) (`KismetSystemLibrary.IsValid` _asbp_base_player))
    (bind _returnvalue (`self.DispenseWeapon`))
    (if (`KismetSystemLibrary.IsValid` _returnvalue)
      (bind _asbp_base_weapon (cast `/Game/CyberSiege/Core/Actors/Weapons/BP_BaseWeapon` _returnvalue))
      (`/Game/CyberSiege/Core/Actors/ActorComponents/BP_WeaponHolster.Replace Weapon` (`/Game/CyberSiege/Core/Actors/Characters/BP_BasePlayer.Weapon Holster` _asbp_base_player) _asbp_base_weapon)
      (`/Game/CyberSiege/Core/Actors/Characters/BP_BasePlayer.Equip Weapon` _asbp_base_player)
      (`/Game/CyberSiege/Core/Actors/ActorComponents/BP_QuestTriggerComponent.Complete Step` (`self.BP_QuestTriggerComponent`)))))

(fn `DispenseWeapon`
  (returns (ReturnValue :type "Actor Object Reference"))
  (if (`KismetSystemLibrary.IsValidClass` (`self.WeaponClass`))
    (bind _returnvalue (`|SpawnActorFromClass` (`self.WeaponClass`) (`KismetMathLibrary.MakeTransform` (9999.0 9999.0 9999.0)) "Undefined" "OverrideRootScale" null null))
    (return _returnvalue)))

(fn `UserConstructionScript`)