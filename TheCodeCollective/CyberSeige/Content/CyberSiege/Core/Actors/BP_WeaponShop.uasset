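; BP_WeaponShop is a weapon shop actor with a sliding door, tied to the wave cycle through BP_WaveManager's begin and end events.
; The door opens at BeginPlay, and OpenDoor and CloseDoor set a direction that Tick uses to lerp it between closed and lowered positions.
; Closing also teleports players inside the box to the arrow's tip, sounding an alarm for each.
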(event `self.ReceiveBeginPlay`
  (bind _output_get (set `self.ClosePosition` (`SceneComponent.K2_GetComponentLocation` (`self.Door`))))
  (set `self.OpenPosition` (- _output_get (0.0 0.0 400.0)))
  (bind _returnvalue (`GameplayStatics.GetActorOfClass` "/Game/CyberSiege/Core/Engine/BP_WaveManager.BP_WaveManager_C"))
  (add `WaveManager.OnWaveEnded` _returnvalue (`|CreateDelegate` :!event `OpenDoor`))
  (add `WaveManager.OnWaveBegin` _returnvalue (`|CreateDelegate` :!event `CloseDoor`))
  (`self.OpenDoor`))

(event `self.ReceiveTick`
  (params (DeltaSeconds :type "Float (single-precision)"))
  (bind _returnvalue (`KismetMathLibrary.FClamp` (+ (`self.DoorAlpha`) (* DeltaSeconds (`self.DoorMoveSpeed`) (`self.DoorDelta`)))))
  (set `self.DoorAlpha` _returnvalue)
  (`SceneComponent.K2_SetWorldLocation` (`self.Door`) (`KismetMathLibrary.VLerp` (`self.OpenPosition`) (`self.ClosePosition`) _returnvalue) false false))

(fn `CloseDoor`
  (bind _arrow (`self.Arrow`))
  (set `self.DoorDelta` 1.0)
  (for _array_element (`PrimitiveComponent.GetOverlappingActors` (`self.Box`) "/Game/CyberSiege/Core/Actors/Characters/BP_BasePlayer.BP_BasePlayer_C")
    (`self.K2_TeleportTo` _array_element (+ (* (`SceneComponent.GetForwardVector` _arrow) (`ArrowComponent.ArrowLength` _arrow)) (`SceneComponent.K2_GetComponentLocation` _arrow)) (`self.K2_GetActorRotation` _array_element))
    (`GameplayStatics.PlaySoundAtLocation` "/Game/CyberSiege/Audio/SFX/AlarmSoundCue.AlarmSoundCue" (`self.K2_GetActorLocation`) (struct) 1.0 1.0 0.0 null null null)))

(fn `OpenDoor`
  (set `self.DoorDelta` -1.0)
  (`GameplayStatics.PlaySoundAtLocation` "/Game/CyberSiege/Audio/SFX/ShopOpenSoundCue.ShopOpenSoundCue" (`self.K2_GetActorLocation`) (struct) 1.0 1.0 0.0 null null null))

(fn `UserConstructionScript`)