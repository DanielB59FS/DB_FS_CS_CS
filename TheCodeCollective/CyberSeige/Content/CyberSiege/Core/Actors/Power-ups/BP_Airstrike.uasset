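; BP_Airstrike is a power-up actor that drops a timed series of bombs, then removes itself.
; BeginPlay waits briefly before enabling drops, then destroys the actor after a longer delay.
; Tick spawns scaled-up BP_Bombs at the BombDropPoint component up to a fixed count, using the CanDropBombs flag and a short Delay to space them out.
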(event `self.ReceiveBeginPlay`
  (`KismetSystemLibrary.Delay` 2.2)
  (set `self.CanDropBombs` true)
  (`KismetSystemLibrary.Delay` 13.0)
  (`self.K2_DestroyActor`))

(event `self.ReceiveTick`
  (params (DeltaSeconds :type "Float (single-precision)"))
  (if (and (`self.CanDropBombs`) (< (`self.BombsDropped`) 10))
    (set `self.CanDropBombs` false)
    (`|SpawnActorFromClass` "/Game/CyberSiege/Core/Actors/Power-ups/BP_Bombs.BP_Bombs_C" (`KismetMathLibrary.MakeTransform` (`SceneComponent.K2_GetComponentLocation` (`self.BombDropPoint`)) (struct) (2.0 2.0 2.0)) "Undefined" "OverrideRootScale" null null)
    (`/Engine/EditorBlueprintResources/StandardMacros.IncrementInt` (`self.BombsDropped`)
      (:`  `
        (`KismetSystemLibrary.Delay` 0.2)
        (set `self.CanDropBombs` true)))))

(fn `UserConstructionScript`)