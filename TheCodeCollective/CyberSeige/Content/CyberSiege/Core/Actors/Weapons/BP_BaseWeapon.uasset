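; Base weapon actor that handles ammo, fire delay and reloading, leaving the Fire event empty for child weapons.
; RequestFire and RequestReload gate on state and broadcast ammo and animation dispatchers.
; FireHitscan traces from the camera, detects headshots by component or bone name, applies damage, reports it to AI and updates GameInstance score and accuracy, ignoring drone capsule hits.
; FireProjectile spawns projectiles from the muzzle socket toward the camera trace point.
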(event `self.ReceiveBeginPlay`
  (set `self.Current Ammo` (`self.Max Ammo`)))

(event `Fire`
  (params (Owner :type "Pawn Object Reference")))

(event `Request Fire`
  (params (Owner :type "Pawn Object Reference"))
  (bind _current_ammo (`self.Current Ammo`))
  (bind _boolean (`self.Can Fire`))
  (if _boolean
    (if (> _current_ammo 0.0)
      (set `self.Current Ammo` (- _current_ammo (`self.Ammo Usage`)))
      (`ActorComponent.Activate` (`self.Particles`) true)
      (`self.Fire` Owner)
      (set `self.CanFire` false)
      (`self.OnAmmoChanged` (`self.Current Ammo`) (`self.Max Ammo`))
      (if (`KismetSystemLibrary.IsValid` (`self.Shoot Animation`))
        (`self.OnShoot` (`self.Shoot Animation`)))
      (`KismetSystemLibrary.K2_SetTimerDelegate` (`|CreateDelegate` :!event `Set Can Fire`) (`self.Delay`))
      (else
        (`self.PlaySound` (`self.FireWithoutAmmoSound`))))))

(event `OnShootAnimationEnded`
  (set `self.Animating` false))

(event `Set Can Fire`
  (set `self.CanFire` true))

(event `Request Reload`
  (if (and (`self.CanFire`) (< (`self.Current Ammo`) (`self.Max Ammo`)))
    (if (`KismetSystemLibrary.IsValid` (`self.Reload Animation`))
      (if (not (`self.Animating`))
        (`self.OnReload` (`self.Reload Animation`))
        (set `self.Animating` true)
        (`self.PlaySound` (`self.ReloadStartSound`)))
      (else
        (`self.Reload`)))))

(event `Reload`
  (bind _output_get (set `self.Current Ammo` (`self.Max Ammo`)))
  (`self.OnAmmoChanged` _output_get (`self.Max Ammo`))
  (set `self.Animating` false)
  (`self.PlaySound` (`self.ReloadEndSound`)))

(fn `Can Fire`
  (returns (Boolean :type Boolean))
  (return (and (`self.CanFire`) (not (`self.Animating`)))))

(fn `Fire Hitscan`
  (params (Owner :type "Pawn Object Reference"))
  (returns (`Out Hit` :type "HitResult Structure") (`Hit Return Value` :type Boolean))
  (locals (`Particle ` :type Boolean))
  (bind _damage (`self.Damage`))
  (bind _returnvalue (`PlayerCameraManager.GetCameraLocation` (`GameplayStatics.GetPlayerCameraManager` 0)))
  (bind (_outhit _returnvalue_2) (`KismetSystemLibrary.LineTraceSingleForObjects` _returnvalue (+ _returnvalue (* (`KismetMathLibrary.GetForwardVector` (`Pawn.GetBaseAimRotation` Owner)) (`self.Range`))) (`self.Object Types`) false (`|MakeArray` null :!type "Actor Object Reference")))
  (bind (_bblockinghit _binitialoverlap _time _distance _location _impactpoint _normal _impactnormal _physmat _hitactor _hitcomponent) (`GameplayStatics.BreakHitResult` _outhit))
  (bind _boolean (message `/Game/CyberSiege/Core/Interfaces/BPI_Enemies.IsEnemy` _hitactor))
  (bind _returnvalue_3 (and _returnvalue_2 _boolean))
  (`/Game/CyberSiege/Core/Engine/BP_GameInstance.UpdateAccuracy` (cast `/Game/CyberSiege/Core/Engine/BP_GameInstance` (`GameplayStatics.GetGameInstance`) :!pure true) _returnvalue_3)
  (if _returnvalue_3
    (bind (_bblockinghit_2 _binitialoverlap_2 _time_2 _distance_2 _location_2 _impactpoint_2 _normal_2 _impactnormal_2 _physmat_2 _hitactor_2 _hitcomponent_2 _hitbonename) (`GameplayStatics.BreakHitResult` _outhit))
    (if (and (or (`KismetStringLibrary.Contains` (`KismetSystemLibrary.GetDisplayName` _hitcomponent_2) "head" false true) (`KismetStringLibrary.Contains` (`KismetStringLibrary.Conv_NameToString` _hitbonename) "head" false true)) _returnvalue_3)
      (`/Game/CyberSiege/Core/Engine/BP_GameInstance.AddScoreValue` (cast `/Game/CyberSiege/Core/Engine/BP_GameInstance` (`GameplayStatics.GetGameInstance`) :!pure true) (`self.HeadShotValue`) "NewEnumerator0")
      (`KismetSystemLibrary.PrintString` "HEADSHOT!!"))
    (if (== (`GameplayStatics.GetObjectClass` _hitactor) "/Game/CyberSiege/Core/Actors/Characters/AI/BP_DroneEnemy.BP_DroneEnemy_C")
      (bind _asbp_drone_enemy (cast `/Game/CyberSiege/Core/Actors/Characters/AI/BP_DroneEnemy` _hitactor)
        (:`then`
          (if (!= (`Character.CapsuleComponent` _asbp_drone_enemy) _hitcomponent)
            (`GameplayStatics.ApplyDamage` _hitactor _damage (`self.GetInstigatorController`) self :!label _label)
            (bind _tags (`Actor.Tags` _hitactor))
            ;[1 1 1] alerting enemies when the get shot
            (for _array_element _tags
              (if (== _array_element "Enemy")
                (`AISense_Damage.ReportDamageEvent` _hitactor self _damage)))
            (`/Game/CyberSiege/Core/Engine/BP_GameInstance.UpdateAccuracy` (cast `/Game/CyberSiege/Core/Engine/BP_GameInstance` (`GameplayStatics.GetGameInstance`) :!pure true) (not (== (`KismetArrayLibrary.Array_Length` _tags) 0)))
            (`GameplayStatics.SpawnEmitterAtLocation` (`self.Impact Particles`) _impactpoint :!label _label_2)
            (else
              (if _returnvalue_2 :!label _label_3
                (goto _label_2)
                (else
                  _))))
          (`GameplayStatics.SpawnSoundAtLocation` (`self.FireWithAmmoSound`) (`self.K2_GetActorLocation`) (struct) 1.0 1.0 0.0 null null)
          (return _outhit _returnvalue_2))
        (:`CastFailed`
          (`KismetSystemLibrary.PrintString` "Drone enemy is not drone enemy (baseWeapon - fire hitscan)")))
      (else
        (goto _label)))
    (else
      (goto _label_3))))

(fn `Fire Projectile`
  (params (Owner :type "Pawn Object Reference"))
  (locals (`End Point` :type "Vector Structure"))
  (bind _returnvalue (`PlayerCameraManager.GetCameraLocation` (`GameplayStatics.GetPlayerCameraManager` 0)))
  (bind _returnvalue_2 (`SceneComponent.GetSocketLocation` (`self.Mesh`) (`self.Fire Pos Socket`)))
  (if (`KismetSystemLibrary.IsValidClass` (`self.Projectile Class`))
    (bind (_outhit _returnvalue_3) (`KismetSystemLibrary.LineTraceSingleForObjects` _returnvalue (+ _returnvalue (* (`KismetMathLibrary.GetForwardVector` (`Pawn.GetBaseAimRotation` Owner)) (`self.Range`))) (`self.Object Types`) false (`|MakeArray` null :!type "Actor Object Reference")))
    (if _returnvalue_3
      (bind _output_get (set `local.End Point` (`.ImpactPoint` (`GameplayStatics.BreakHitResult` _outhit))))
      (else
        (set `local.End Point` (`.TraceEnd` (`GameplayStatics.BreakHitResult` _outhit)))))
    (bind _returnvalue_4 (`KismetMathLibrary.Normal` (- _output_get _returnvalue_2)))
    (`|SpawnActorFromClass` (`self.Projectile Class`) (`KismetMathLibrary.MakeTransform` (+ (* _returnvalue_4 100.0) _returnvalue_2) (`KismetMathLibrary.MakeRotFromX` _returnvalue_4)) "Undefined" "OverrideRootScale" null null)
    (`GameplayStatics.SpawnSoundAtLocation` (`self.FireWithAmmoSound`) (`self.K2_GetActorLocation`) (struct) 1.0 1.0 0.0 null null)
    (else
      (`KismetSystemLibrary.PrintString` "No Projectile Set for Wepaon"))))

(fn `Get Aim Dir`
  (params (Owner :type "Pawn Object Reference"))
  (returns (`Out Hit Location` :type "Vector Structure"))
  (return (+ (`PlayerCameraManager.GetCameraLocation` (`GameplayStatics.GetPlayerCameraManager` 0)) (* (`KismetMathLibrary.GetForwardVector` (`Pawn.GetBaseAimRotation` Owner)) (`self.Range`)))))

(fn `GetEnemyCount`
  (returns (EnemyCount :type Integer))
  (return 0))

(fn `GetLHSLocation`
  (returns (LeftHandSocket :type "Vector Structure"))
  (return (0.0 0.0 0.0)))

(fn `IsEnemy`
  (returns (Boolean :type Boolean))
  (return false))

(fn `PlaySound`
  (params (Sound :type "SoundCue Object Reference"))
  (bind _audio (`self.Audio`))
  (if (`KismetSystemLibrary.IsValid` Sound)
    (`AudioComponent.SetSound` _audio Sound)
    (`AudioComponent.SetPitchMultiplier` _audio (`KismetMathLibrary.RandomFloatInRange` 1.0 10.0)))
  (`AudioComponent.Play` _audio 0.0)
  (`AudioComponent.SetPitchMultiplier` _audio 1.0))

(fn `UserConstructionScript`)