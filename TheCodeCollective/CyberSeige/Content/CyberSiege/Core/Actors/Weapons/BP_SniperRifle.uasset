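; Sniper rifle weapon that fires a hitscan shot and draws a Niagara beam trail.
; On Fire, it runs FireHitscan for the owner and takes the impact point as the trail end, or the GetAimDir result on a miss.
; It spawns NS_SniperTrail inactive at the mesh's fire socket, sets its BeamEnd variable, then activates it.
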(event `self.Fire`
  (params (Owner :type "Pawn Object Reference"))
  (bind (_out_hit _hit_return_value) (`self.Fire Hitscan` Owner))
  (bind _out_hit_location (`self.Get Aim Dir` Owner))
  (if _hit_return_value
    (set `self.TracerEnd` (`.ImpactPoint` (`GameplayStatics.BreakHitResult` _out_hit)))
    (else
      (set `self.TracerEnd` _out_hit_location)))
  (bind _returnvalue (`NiagaraFunctionLibrary.SpawnSystemAtLocation` "/Game/CyberSiege/Art/NS_SniperTrail.NS_SniperTrail" (`SceneComponent.GetSocketLocation` (`self.Mesh`) (`self.Fire Pos Socket`)) (struct) (1.0 1.0 1.0) true false))
  (`NiagaraComponent.SetVariableVec3` _returnvalue "BeamEnd" (`self.TracerEnd`))
  (`ActorComponent.Activate` _returnvalue true))

(fn `UserConstructionScript`
  (`parent.UserConstructionScript`))