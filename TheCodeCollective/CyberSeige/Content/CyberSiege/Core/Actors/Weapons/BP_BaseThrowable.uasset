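; Base throwable projectile actor that plays a throw sound on spawn and ends by spawning an effect actor at its sphere's location, then destroying itself.
; An ExplodeOnImpact flag picks whether the effect fires on the first projectile bounce or after a delay from BeginPlay.
; Delayed throwables play a surface sound on bounce, throttled by a DoOnce and a short timer.
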(event `self.ReceiveBeginPlay`
  (`GameplayStatics.PlaySoundAtLocation` (`self.ThrowSound`) (`self.K2_GetActorLocation`) (struct) 1.0 1.0 0.0 null null null)
  (if (not (`self.ExplodeOnImpact`))
    (`KismetSystemLibrary.Delay` (`self.Delay`))
    (`self.Spawn Effect`)))

(event `self.ProjectileMovement.OnProjectileBounce`
  (params (ImpactResult :type "HitResult Structure (by ref)") (ImpactVelocity :type "Vector Structure (by ref)"))
  (`/Engine/EditorBlueprintResources/StandardMacros.DoOnce` false :!label _label
    (:`Completed`
      (if (`self.ExplodeOnImpact`)
        (`self.Spawn Effect`)
        (else
          (`GameplayStatics.PlaySoundAtLocation` (`self.SurfaceBounceSound`) (`self.K2_GetActorLocation`) (struct) 1.0 1.0 0.0 null null null)
          (`KismetSystemLibrary.K2_SetTimerDelegate` (`|CreateDelegate` :!event `Reset Bounce Sound`) 0.15))))))

(event `Reset Bounce Sound`
  (goto _label :!via `Reset`))

(event `Spawn Effect`
  (`|SpawnActorFromClass` (`self.Effect`) (`KismetMathLibrary.MakeTransform` (`SceneComponent.K2_GetComponentLocation` (`self.Sphere`))) "Undefined" "OverrideRootScale" null null)
  (`self.K2_DestroyActor`))

(fn `UserConstructionScript`)