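; BP_WeaponShopDisplay is a weapon shop display actor that shows a floating, spinning hologram of weapons.
; Tick spins the Weapon skeletal mesh on yaw and bobs it vertically with per-frame cosine offsets driven by an accumulated float time.
; BeginPlay starts a looping timer, presumably bound to SwitchMesh, which cycles through the WeaponMeshes array and reapplies the hologram material.
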(event `self.ReceiveBeginPlay`
  (`KismetSystemLibrary.K2_SetTimerDelegate` (`|CreateDelegate` :!event `SwitchMesh`) 3.5 true))

(event `self.ReceiveTick`
  (params (DeltaSeconds :type "Float (single-precision)"))
  (bind _returnvalue (+ (`self.FloatDelta`) (* DeltaSeconds (`self.FloatDirection`) (`self.FloatSpeed`))))
  (bind _returnvalue_2 (`KismetMathLibrary.Cos` _returnvalue))
  (set `self.FloatDelta` _returnvalue)
  (if (> _returnvalue_2 6.28)
    (set `self.FloatDirection` -1.0)
    (elif (< _returnvalue_2 -1.0)
      (set `self.FloatDirection` -1.0)))
  (`SceneComponent.K2_AddWorldOffset` (`self.Weapon`) (`KismetMathLibrary.MakeVector` 0.0 0.0 (/ _returnvalue_2 3.0)) false false)
  (`SceneComponent.K2_AddWorldRotation` (`self.Weapon`) (`KismetMathLibrary.MakeRotator` 0.0 0.0 (* DeltaSeconds (`self.RotateSpeed`))) false false))

(fn `SwitchMesh`
  (bind _result (`/Engine/EditorBlueprintResources/StandardMacros.IncrementInt` (`self.Index`))
    (:`  `
      (if (>= _result (`KismetArrayLibrary.Array_Length` (`self.WeaponMeshes`)))
        (bind _output_get (set `self.Index` 0)))
      (`SkinnedMeshComponent.SetSkinnedAssetAndUpdate` (`self.Weapon`) (`|GetArrayItem` (`self.WeaponMeshes`) _output_get) false)
      (`PrimitiveComponent.SetMaterial` (`self.Weapon`) 0 "/Game/CyberSiege/Art/MI_WeaponHologram.MI_WeaponHologram"))))

(fn `UserConstructionScript`)