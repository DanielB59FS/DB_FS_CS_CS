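; BP_Platform is a destructible defense platform actor with a health component and a friendly health bar widget.
; Every Tick it sets the bar to the clamped current-to-max health ratio and rotates the widget to face player 0's camera.
; It then destroys itself once health reaches zero, polling each frame rather than reacting to a damage or death event.
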(event `self.ReceiveTick`
  (params (DeltaSeconds :type "Float (single-precision)"))
  (`self.UpdateHealthBar`)
  (if (<= (`/Game/CyberSiege/Core/Actors/ActorComponents/BP_HealthComponent.CurrentHealth` (`self.BP_HealthComponent`)) 0.0)
    (`self.K2_DestroyActor`)))

(fn `UpdateHealthBar`
  (bind _bp_healthcomponent (`self.BP_HealthComponent`))
  (bind _health_bar_widget (`self.Health Bar Widget`))
  (bind _aswbp_health_bar_friendly (cast `/Game/CyberSiege/Core/Widgets/WBP_HealthBar_Friendly` (`WidgetComponent.GetWidget` (`self.Health Bar Widget`))))
  (`ProgressBar.SetPercent` (`/Game/CyberSiege/Core/Widgets/WBP_HealthBar_Friendly.HealthBar` _aswbp_health_bar_friendly) (`KismetMathLibrary.FClamp` (/ (`/Game/CyberSiege/Core/Actors/ActorComponents/BP_HealthComponent.CurrentHealth` _bp_healthcomponent) (`/Game/CyberSiege/Core/Actors/ActorComponents/BP_HealthComponent.MaxHealth` _bp_healthcomponent))))
  (`SceneComponent.K2_SetWorldRotation` _health_bar_widget (`KismetMathLibrary.FindLookAtRotation` (`SceneComponent.K2_GetComponentLocation` _health_bar_widget) (`SceneComponent.K2_GetComponentLocation` (`PlayerCameraManager.TransformComponent` (`GameplayStatics.GetPlayerCameraManager` 0)))) false false))

(fn `UserConstructionScript`)