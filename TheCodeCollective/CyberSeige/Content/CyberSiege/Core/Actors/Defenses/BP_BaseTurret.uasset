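; Base turret defense for CyberSiege: a friendly, twin-barrel actor with health, player-paid repairs and per-barrel recoil animation.
; Tick turns the health bar and cost text toward the camera, drops dead targets and flags death at zero health.
; Interact applies the scrap cost through the player's BuildComponent, flags repairing and advances a quest step.
; It also exposes a heal function, a scrap affordability check and a clamped enemy counter.
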(event `self.FireAnimationR`
  (`TimelineComponent.PlayFromStart` (`self.RecoilTimelineR`)))

(event `self.FireAnimationL`
  (`TimelineComponent.PlayFromStart` (`self.RecoilTimelineL`)))

(event `self.ReceiveTick`
  (params (DeltaSeconds :type "Float (single-precision)"))
  (bind _target (`self.Target`))
  (set `self.Health` (`/Game/CyberSiege/Core/Actors/ActorComponents/BP_HealthComponent.CurrentHealth` (`self.BP_HealthComponent`)))
  (if (not (`self.IsDead`))
    (`self.UpdateHealthBar`)
    (if (`KismetSystemLibrary.IsValid` _target)
      (bind _asbp_base_enemy_1 (cast `/Game/CyberSiege/Core/Actors/Characters/AI/BP_BaseEnemy1` _target))
      (if (`/Game/CyberSiege/Core/Actors/Characters/AI/BP_BaseEnemy1.IsDead` _asbp_base_enemy_1)
        (set `self.Target` null)))
    (if (<= (`/Game/CyberSiege/Core/Actors/ActorComponents/BP_HealthComponent.CurrentHealth` (`self.BP_HealthComponent`)) 0.0)
      (set `self.IsDead` true))))

(event `/Game/CyberSiege/Core/Interfaces/BPI_Enemies.DecrementEnemyCount`
  (bind _result (`/Engine/EditorBlueprintResources/StandardMacros.DecrementInt` (`self.EnemyCount`))
    (:`  `
      (set `self.EnemyCount` (`KismetMathLibrary.Clamp` _result 0 4)))))

(event `/Game/CyberSiege/Core/Interfaces/BPI_Interact.Interact`
  (params (`Interacting Actor` :type "Actor Object Reference"))
  (if (and (`self.bTargetedByPlayer`) (`self.bPlayerCanAfford`))
    (bind _result (`/Engine/EditorBlueprintResources/StandardMacros.NegateInt` (`self.RepairCost`))
      (:`  `
        (bind _asbp_base_player (cast `/Game/CyberSiege/Core/Actors/Characters/BP_BasePlayer` (`self.Player`)))
        (`/Game/CyberSiege/Core/Actors/ActorComponents/BP_BuildComponent.ChangeScrapCount` (`/Game/CyberSiege/Core/Actors/Characters/BP_BasePlayer.Build Component` _asbp_base_player) _result)
        (`SceneComponent.SetVisibility` (`self.TextRenderer`) false true)
        (set `self.Repairing` true)
        (`/Game/CyberSiege/Core/Actors/ActorComponents/BP_QuestTriggerComponent.Complete Step` (`self.QuestTrigger`))))))

(event `/Game/CyberSiege/Core/Interfaces/BPI_Enemies.IncrementEnemyCount`
  (bind _result (`/Engine/EditorBlueprintResources/StandardMacros.IncrementInt` (`self.EnemyCount`))
    (:`  `
      (set `self.EnemyCount` (`KismetMathLibrary.Clamp` _result 0 4)))))

(event `self.ReceiveBeginPlay`
  (`parent.ReceiveBeginPlay`)
  (set `self.MaxHealth` (`KismetMathLibrary.FTrunc` (`/Game/CyberSiege/Core/Actors/ActorComponents/BP_HealthComponent.MaxHealth` (`self.BP_HealthComponent`))))
  (`TimelineComponent.SetFloatCurve` (`self.RecoilTimelineR`) "/Game/CyberSiege/Core/Actors/Defenses/Misc/RecoilCurve1.RecoilCurve1" "Recoil")
  (`TimelineComponent.SetFloatCurve` (`self.RecoilTimelineL`) "/Game/CyberSiege/Core/Actors/Defenses/Misc/RecoilCurve1.RecoilCurve1" "Recoil"))

(fn `CheckPlayerScrap`
  (params (cost :type Integer))
  (returns (ReturnValue :type Boolean))
  (bind _textrenderer (`self.TextRenderer`))
  (`TextRenderComponent.K2_SetText` (`self.TextRenderer`) (`KismetTextLibrary.Conv_StringToText` (`KismetStringLibrary.Conv_IntToString` cost)))
  (bind _asbp_base_player (cast `/Game/CyberSiege/Core/Actors/Characters/BP_BasePlayer` (`self.Player`)))
  (bind _newparam (`/Game/CyberSiege/Core/Actors/ActorComponents/BP_BuildComponent.GetScrapCount` (`/Game/CyberSiege/Core/Actors/Characters/BP_BasePlayer.Build Component` _asbp_base_player)))
  (bind _returnvalue (> _newparam cost))
  (if _returnvalue
    (`TextRenderComponent.SetTextRenderColor` _textrenderer (`self.Green`))
    (else
      (`TextRenderComponent.SetTextRenderColor` _textrenderer (`self.Red`))
      (`SceneComponent.SetVisibility` (`self.TextRendererNot`) true false)))
  (return _returnvalue))

(fn `GetEnemyCount`
  (returns (EnemyCount :type Integer))
  (return (`self.EnemyCount`)))

(fn `GetLHSLocation`
  (returns (LeftHandSocket :type "Vector Structure"))
  (return (0.0 0.0 0.0)))

(fn `Heal`
  (params (DeltaTime :type "Float (double-precision)"))
  (bind _bp_healthcomponent (`self.BP_HealthComponent`))
  (set `/Game/CyberSiege/Core/Actors/ActorComponents/BP_HealthComponent.CurrentHealth` (+ (* DeltaTime 10.0) (`/Game/CyberSiege/Core/Actors/ActorComponents/BP_HealthComponent.CurrentHealth` _bp_healthcomponent)) _bp_healthcomponent)
  (return))

(fn `IsEnemy`
  (returns (Boolean :type Boolean))
  (return false))

(fn `UpdateHealthBar`
  (bind _bp_healthcomponent (`self.BP_HealthComponent`))
  (bind _textrenderer (`self.TextRenderer`))
  (bind _health_bar_widget (`self.Health Bar Widget`))
  (bind _aswbp_health_bar_friendly (cast `/Game/CyberSiege/Core/Widgets/WBP_HealthBar_Friendly` (`WidgetComponent.GetWidget` (`self.Health Bar Widget`))))
  (`ProgressBar.SetPercent` (`/Game/CyberSiege/Core/Widgets/WBP_HealthBar_Friendly.HealthBar` _aswbp_health_bar_friendly) (`KismetMathLibrary.FClamp` (/ (`/Game/CyberSiege/Core/Actors/ActorComponents/BP_HealthComponent.CurrentHealth` _bp_healthcomponent) (`/Game/CyberSiege/Core/Actors/ActorComponents/BP_HealthComponent.MaxHealth` _bp_healthcomponent))))
  (`SceneComponent.K2_SetWorldRotation` _health_bar_widget (`KismetMathLibrary.FindLookAtRotation` (`SceneComponent.K2_GetComponentLocation` _health_bar_widget) (`SceneComponent.K2_GetComponentLocation` (`PlayerCameraManager.TransformComponent` (`GameplayStatics.GetPlayerCameraManager` 0)))) false false)
  (`SceneComponent.K2_SetWorldRotation` _textrenderer (`KismetMathLibrary.FindLookAtRotation` (`SceneComponent.K2_GetComponentLocation` _textrenderer) (`SceneComponent.K2_GetComponentLocation` (`PlayerCameraManager.TransformComponent` (`GameplayStatics.GetPlayerCameraManager` 0)))) false false))

(fn `UserConstructionScript`)