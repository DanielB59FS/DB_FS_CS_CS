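; BP_LaserFence is a defense actor representing a laser fence that is removed from the game when its health runs out.
; Tick polls the BPHealthComponent's current health every frame instead of reacting to an event.
; At zero or below, it deactivates each of its three valid laser particle components, then destroys the actor.
; The graph contains no damage, overlap or construction logic.
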(event `self.ReceiveTick`
  (params (DeltaSeconds :type "Float (single-precision)"))
  (bind _laserpscomponent1 (`self.LaserPSComponent1`))
  (bind _laserpscomponent2 (`self.LaserPSComponent2`))
  (bind _laserpscomponent3 (`self.LaserPSComponent3`))
  (if (<= (`/Game/CyberSiege/Core/Actors/ActorComponents/BP_HealthComponent.CurrentHealth` (`self.BP_HealthComponent`)) 0.0)
    (if (`KismetSystemLibrary.IsValid` _laserpscomponent1)
      (`ActorComponent.Deactivate` _laserpscomponent1))
    (if (`KismetSystemLibrary.IsValid` _laserpscomponent2)
      (`ActorComponent.Deactivate` _laserpscomponent2))
    (if (`KismetSystemLibrary.IsValid` _laserpscomponent3)
      (`ActorComponent.Deactivate` _laserpscomponent3))
    (`self.K2_DestroyActor`)))

(fn `UserConstructionScript`)