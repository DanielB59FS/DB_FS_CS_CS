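; Destructible defense blockade that spider enemies leap over, destroying itself when its health component runs out.
; Front and back trigger boxes launch living spiders toward the opposite box, using a projectile-motion velocity solved for a set duration.
; Per-side spider arrays detect arrivals from the other side, clearing CanJump, which this graph never re-enables.
; It also binds to the wave game mode's round-end event and keeps a clamped enemy count.
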(event `self.ReceiveBeginPlay`
  (bind _returnvalue (`GameplayStatics.GetGameMode`))
  (if (== (`GameplayStatics.GetObjectClass` _returnvalue) "/Game/CyberSiege/Core/GameModes/BP_WaveGameMode.BP_WaveGameMode_C")
    (bind _asbp_wave_game_mode (cast `/Game/CyberSiege/Core/GameModes/BP_WaveGameMode` _returnvalue))
    (add `/Game/CyberSiege/Core/GameModes/BP_WaveGameMode.OnRoundEnded` _asbp_wave_game_mode (`|CreateDelegate` :!event `ResetSpiderArrays`))))

(event `self.ReceiveTick`
  (params (DeltaSeconds :type "Float (single-precision)"))
  (if (<= (`/Game/CyberSiege/Core/Actors/ActorComponents/BP_HealthComponent.CurrentHealth` (`self.BP_HealthComponent`)) 0.0)
    (`self.K2_DestroyActor`)))

(event `/Game/CyberSiege/Core/Interfaces/BPI_Enemies.DecrementEnemyCount`
  (bind _result (`/Engine/EditorBlueprintResources/StandardMacros.DecrementInt` (`self.EnemyCount`))
    (:`  `
      (set `self.EnemyCount` (`KismetMathLibrary.Clamp` _result 0 3)))))

(event `/Game/CyberSiege/Core/Interfaces/BPI_Enemies.IncrementEnemyCount`
  (bind _result (`/Engine/EditorBlueprintResources/StandardMacros.IncrementInt` (`self.EnemyCount`))
    (:`  `
      (set `self.EnemyCount` (`KismetMathLibrary.Clamp` _result 0 3)))))

(event `self.JumpingBoxFront.OnComponentBeginOverlap`
  (params (OverlappedComponent :type "PrimitiveComponent Object Reference") (OtherActor :type "Actor Object Reference") (OtherComp :type "PrimitiveComponent Object Reference") (OtherBodyIndex :type Integer) (bFromSweep :type Boolean) (SweepResult :type "HitResult Structure (by ref)"))
  (if (== (`GameplayStatics.GetObjectClass` OtherActor) "/Game/CyberSiege/Core/Actors/Characters/AI/BP_SpiderEnemy.BP_SpiderEnemy_C")
    (for _array_element (`self.SpiderArrayBack`)
      (if (== OtherActor _array_element)
        (set `self.CanJump` false)))
    (if (`self.CanJump`)
      (bind _asbp_spider_enemy (cast `/Game/CyberSiege/Core/Actors/Characters/AI/BP_SpiderEnemy` OtherActor))
      (if (not (`/Game/CyberSiege/Core/Actors/Characters/AI/BP_BaseEnemy1.IsDead` _asbp_spider_enemy))
        (`KismetArrayLibrary.Array_AddUnique` (`self.SpiderArrayFront`) _asbp_spider_enemy)
        (bind _launchvector (`self.CalculateLaunch` (`SceneComponent.K2_GetComponentLocation` (`self.JumpingBoxBack`)) (`self.K2_GetActorLocation` _asbp_spider_enemy) (`self.LaunchDuration`)))
        (`Character.LaunchCharacter` _asbp_spider_enemy _launchvector true true)))))

(event `self.JumpingBoxBack.OnComponentBeginOverlap`
  (params (OverlappedComponent :type "PrimitiveComponent Object Reference") (OtherActor :type "Actor Object Reference") (OtherComp :type "PrimitiveComponent Object Reference") (OtherBodyIndex :type Integer) (bFromSweep :type Boolean) (SweepResult :type "HitResult Structure (by ref)"))
  (if (== (`GameplayStatics.GetObjectClass` OtherActor) "/Game/CyberSiege/Core/Actors/Characters/AI/BP_SpiderEnemy.BP_SpiderEnemy_C")
    (for _array_element (`self.SpiderArrayFront`)
      (if (== OtherActor _array_element)
        (set `self.CanJump` false)))
    (if (`self.CanJump`)
      (bind _asbp_spider_enemy (cast `/Game/CyberSiege/Core/Actors/Characters/AI/BP_SpiderEnemy` OtherActor))
      (if (not (`/Game/CyberSiege/Core/Actors/Characters/AI/BP_BaseEnemy1.IsDead` _asbp_spider_enemy))
        (`KismetArrayLibrary.Array_AddUnique` (`self.SpiderArrayBack`) _asbp_spider_enemy)
        (bind _launchvector (`self.CalculateLaunch` (`SceneComponent.K2_GetComponentLocation` (`self.JumpingBoxFront`)) (`self.K2_GetActorLocation` _asbp_spider_enemy) (`self.LaunchDuration`)))
        (`Character.LaunchCharacter` _asbp_spider_enemy _launchvector true true)))))

(event `ResetSpiderArrays`
  (`KismetArrayLibrary.Array_Clear` (`self.SpiderArrayFront`))
  (`KismetArrayLibrary.Array_Clear` (`self.SpiderArrayBack`)))

(fn `CalculateLaunch`
  (params (EndPoint :type "Vector Structure") (StartPoint :type "Vector Structure") (Duration :type "Float (double-precision)"))
  (returns (LaunchVector :type "Vector Structure"))
  (bind _launchduration (`self.LaunchDuration`))
  (set `self.LaunchDuration` Duration)
  (return (`KismetMathLibrary.MakeVector` (/ (- (.x EndPoint) (.x StartPoint)) _launchduration) (/ (- (.y EndPoint) (.y StartPoint)) _launchduration) (/ (- (.z EndPoint) (+ (.z StartPoint) (* (`KismetMathLibrary.Square` (`self.LaunchDuration`)) -0.5 982.0))) _launchduration))))

(fn `GetEnemyCount`
  (returns (EnemyCount :type Integer))
  (return (`self.EnemyCount`)))

(fn `GetLHSLocation`
  (returns (LeftHandSocket :type "Vector Structure"))
  (return (0.0 0.0 0.0)))

(fn `IsEnemy`
  (returns (Boolean :type Boolean))
  (return false))

(fn `UserConstructionScript`)