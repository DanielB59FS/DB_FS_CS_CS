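; BP_Castle is the stationary castle whose destruction loses the game.
; It binds a handler to its health component's change event on BeginPlay and caches the player character.
; Tick polls current health and, at zero or below, tells BP_WaveGameMode to end the game with a loss message, printing a warning if the mode differs.
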(event `self.ReceiveBeginPlay`
  (bind _asbp_base_player (cast `/Game/CyberSiege/Core/Actors/Characters/BP_BasePlayer` (`GameplayStatics.GetPlayerCharacter` 0)))
  (add `/Game/CyberSiege/Core/Actors/ActorComponents/BP_HealthComponent.OnHealthChanged` (`self.BP_HealthComponent`) (`|CreateDelegate` (`/Game/CyberSiege/Core/Actors/Characters/BP_BasePlayer.Get Gameplay HUD` _asbp_base_player) :!event `SetCastleHealth`)))

(event `self.ReceiveTick`
  (params (DeltaSeconds :type "Float (single-precision)"))
  ;[1 1 1] Converted to code
  (if (<= (`/Game/CyberSiege/Core/Actors/ActorComponents/BP_HealthComponent.CurrentHealth` (`self.BP_HealthComponent`)) 0.0)
    (bind _asbp_wave_game_mode (cast `/Game/CyberSiege/Core/GameModes/BP_WaveGameMode` (`GameplayStatics.GetGameMode`))
      (:`then`
        (`/Game/CyberSiege/Core/GameModes/BP_WaveGameMode.GameEnded` _asbp_wave_game_mode "You Lost! \nCastle Destroyed"))
      (:`CastFailed`
        (`KismetSystemLibrary.PrintString` "Game Mode is not BP_DefaultGameMode (BP_Castle)")))))

(fn `UserConstructionScript`)