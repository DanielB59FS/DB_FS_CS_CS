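; Health pickup actor that restores a fixed fraction of a player's max health.
; Tick spins the mesh by game time and bobs it by adding a sine offset to its current height each frame.
; Sphere overlap accepts only the exact BP_BasePlayer class below full health, writes clamped health to its HealthComponent and notifies the change.
; Once used, it destroys itself and any attach parent actor.
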(event `self.ReceiveBeginPlay`)

(event `self.ReceiveTick`
  (params (DeltaSeconds :type "Float (single-precision)"))
  (bind _returnvalue (`self.GetGameTimeSinceCreation`))
  (bind _staticmesh (`self.StaticMesh`))
  (`SceneComponent.K2_SetWorldLocationAndRotation` _staticmesh (`KismetMathLibrary.MakeVector` (.x (`SceneComponent.K2_GetComponentLocation` _staticmesh)) (.y (`SceneComponent.K2_GetComponentLocation` _staticmesh)) (+ (.z (`SceneComponent.K2_GetComponentLocation` _staticmesh)) (* (`KismetMathLibrary.DegSin` (* _returnvalue (`self.BobSpeed`))) (`self.BobHeight`)))) (`KismetMathLibrary.MakeRotator` 0.0 0.0 (* _returnvalue (`self.SpinSpeed`))) false false))

(event `self.Sphere.OnComponentBeginOverlap`
  (params (OverlappedComponent :type "PrimitiveComponent Object Reference") (OtherActor :type "Actor Object Reference") (OtherComp :type "PrimitiveComponent Object Reference") (OtherBodyIndex :type Integer) (bFromSweep :type Boolean) (SweepResult :type "HitResult Structure (by ref)"))
  (bind _returnvalue (`self.GetAttachParentActor`))
  (if (== (`GameplayStatics.GetObjectClass` OtherActor) "/Game/CyberSiege/Core/Actors/Characters/BP_BasePlayer.BP_BasePlayer_C")
    (bind _asbp_base_player (cast `/Game/CyberSiege/Core/Actors/Characters/BP_BasePlayer` OtherActor))
    (bind _healthcomponent (`/Game/CyberSiege/Core/Actors/Characters/BP_BasePlayer.HealthComponent` _asbp_base_player))
    (bind _currenthealth (`/Game/CyberSiege/Core/Actors/ActorComponents/BP_HealthComponent.CurrentHealth` _healthcomponent))
    (bind _maxhealth (`/Game/CyberSiege/Core/Actors/ActorComponents/BP_HealthComponent.MaxHealth` _healthcomponent))
    (if (< _currenthealth _maxhealth)
      (bind _output_get (set `/Game/CyberSiege/Core/Actors/ActorComponents/BP_HealthComponent.CurrentHealth` (`KismetMathLibrary.FClamp` (+ _currenthealth (* _maxhealth 0.15)) 0.0 _maxhealth) _healthcomponent))
      (`/Game/CyberSiege/Core/Actors/ActorComponents/BP_HealthComponent.OnHealthChanged` _healthcomponent (/ _output_get _maxhealth))
      (if (`KismetSystemLibrary.IsValid` _returnvalue)
        (`self.K2_DestroyActor` _returnvalue))
      (`self.K2_DestroyActor`))))

(fn `UserConstructionScript`)