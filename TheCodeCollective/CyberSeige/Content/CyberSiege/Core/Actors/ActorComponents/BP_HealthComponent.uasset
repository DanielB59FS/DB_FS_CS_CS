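; BP_HealthComponent is an actor component that tracks its owner's health through the OnTakeAnyDamage event.
; A first Shock_DT hit starts the shock effect instead of subtracting health; hits while shocked deal double damage until OnShockEffectEnded.
; The Temp macro gates health loss on positive damage and CanBeDamaged.
; Dispatchers report normalized health for damage, healing, death and changes, and death unbinds the damage handler.
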(event `self.ReceiveBeginPlay`
  ;[1 1 1] In Code
  (set `self.CurrentHealth` (`self.MaxHealth`))
  (add `Actor.OnTakeAnyDamage` (`self.GetOwner`) (`|CreateDelegate` :!event `HandleDamage`)))

(event `HandleDamage`
  (params (DamagedActor :type "Actor Object Reference") (Damage :type "Float (double-precision)") (DamageType :type "DamageType Object Reference") (InstigatedBy :type "Controller Object Reference") (DamageCauser :type "Actor Object Reference"))
  (bind _returnvalue (/ (`self.CurrentHealth`) (`self.MaxHealth`)))
  (bind _returnvalue_2 (* Damage (`self.DamageMultiplier`)))
  ;[1 1 1] In Code
  (bind _asshock_dt (cast `Shock_DT` DamageType)
    (:`then`
      (if (not (`self.IsShocked`))
        (`EffectsInterface.StartEffect` _asshock_dt DamagedActor DamageCauser Damage)
        (set `self.IsShocked` true)
        (else
          (if (`self.IsShocked`) :!label _label
            (set `self.DamageMultiplier` 2.0)
            (else
              (set `self.DamageMultiplier` 1.0)))
          (`self.Temp` DamagedActor _returnvalue_2
            (:`then`
              (bind _output_get (set `self.CurrentHealth` (`KismetMathLibrary.FClamp` (- (`self.CurrentHealth`) _returnvalue_2) 0.0 (`self.MaxHealth`)))))
            (:`else`
              _))
          (if (> _output_get 0.0)
            (if (> _returnvalue_2 0.0)
              (`self.OnDamaged` _returnvalue)
              (else
                (`self.OnHealed` _returnvalue)))
            (else
              (remove `Actor.OnTakeAnyDamage` (`self.GetOwner`) (`|CreateDelegate` :!event `HandleDamage`))
              (`self.OnDeath` 0.0)))
          (`self.OnHealthChanged` (/ (`self.CurrentHealth`) (`self.MaxHealth`))))))
    (:`CastFailed`
      (goto _label))))

(event `On Shock Effect Ended`
  ;[1 1 1] In Code
  (set `self.IsShocked` false))