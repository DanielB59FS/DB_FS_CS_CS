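; Player build component for placing defenses, driven by a build state that routes clicks and scrolling to event dispatchers or to placement and rotation.
; While placing, a preview mesh follows a camera trace, snaps to turret platform sockets and tints red or green from a box overlap and cost check.
; Placing spawns the defense with a builder drone, spends scrap from the balance it tracks and links teleporters to unpartnered ones.
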(event `self.ReceiveBeginPlay`
  (`self.ChangeScrapCount` 250))

(event `self.ReceiveTick`
  (params (DeltaSeconds :type "Float (single-precision)"))
  (if (and (`self.Active`) (`|EnumEquality` (`self.Build State`) "NewEnumerator2"))
    (if (!= (`KismetSystemLibrary.IsValid` (`self.Placeable Preview Object`)) false)
      (`self.Update Placeable Preview`)
      (else
        (bind _returnvalue (`|SpawnActorFromClass` (`self.SelectedDefense`) (`KismetMathLibrary.MakeTransform` (-9999.0 -9999.0 -9999.0)) "Undefined" "OverrideRootScale" null null))
        (bind _returnvalue_2 (`|SpawnActorFromClass` (`self.Placeable Preview Class`) (`KismetMathLibrary.MakeTransform` (0.0 0.0 0.0)) "Undefined" "OverrideRootScale" null null))
        (`StaticMeshComponent.SetStaticMesh` (`/Game/Sandboxes/Chadwick/BP_PlaceablePreview.Mesh` _returnvalue_2) (`Defenses.WholeMesh` _returnvalue))
        (set `self.Bounding Box Extents` (`BoxComponent.BoxExtent` (`Defenses.BoundingBox` _returnvalue)))
        (set `self.Placeable Preview Object` _returnvalue_2)
        (bind _returnvalue_3 (`KismetMaterialLibrary.CreateDynamicMaterialInstance` "/Game/Sandboxes/Chadwick/M_TransparentRed.M_TransparentRed"))
        (set `self.Dynamic Material` _returnvalue_3)
        (bind _outactors (`GameplayStatics.GetAllActorsOfClass` (`self.Placeable Preview Class`)))
        (`PrimitiveComponent.SetMaterial` (`/Game/Sandboxes/Chadwick/BP_PlaceablePreview.Mesh` (`|GetArrayItem` _outactors)) 0 (`self.Dynamic Material`))
        (`Actor.K2_DestroyActor` _returnvalue)))
    (elif (`KismetSystemLibrary.IsValid` (`self.Placeable Preview Object`))
      (`Actor.K2_DestroyActor` (`self.Placeable Preview Object`)))))

(fn `ChangeScrapCount`
  (params (`Change Amount` :type Integer))
  (bind _output_get (set `self.ScrapCount` (+ (`self.ScrapCount`) `Change Amount`)))
  (`self.OnScrapCountChanged` _output_get))

(fn `FindPartnerTeleporter`
  (params (FirstTeleporter :type "Teleporter Object Reference"))
  (bind _outactors (`GameplayStatics.GetAllActorsOfClass` "/Script/CyberSeige.Teleporter"))
  (for _array_element _outactors
    (if (and (== (`Teleporter.PartnerTeleporter` _array_element) null) (!= _array_element (`local.FirstTeleporter`)))
      (bind _output_get (set `Teleporter.PartnerTeleporter` (`local.FirstTeleporter`) _array_element))
      (set `Teleporter.PartnerTeleporter` _array_element _output_get)
      (`KismetSystemLibrary.PrintString` "Teleporters Linked!"))))

(fn `GetScrapCount`
  (returns (NewParam :type Integer))
  (return (`self.ScrapCount`)))

(fn `Left Click`
  (switch `/Game/CyberSiege/Core/Actors/ActorComponents/EBuildStates` (`self.Build State`)
    (:`NewEnumerator0`
      (`self.OnLeftClick` :!label _label))
    (:`NewEnumerator1`
      (goto _label))
    (:`NewEnumerator2`
      (`self.Place Placeable`))))

(fn `Place Placeable`
  (bind _placeable_preview_object (`self.Placeable Preview Object`))
  (bind _returnvalue (`PlayerCameraManager.GetCameraLocation` (`GameplayStatics.GetPlayerCameraManager` 0)))
  (if (`self.Placement Valid`)
    (bind _aspawn (cast `Pawn` (`self.GetOwner`)))
    (bind (_outhit _returnvalue_2) (`KismetSystemLibrary.LineTraceSingleForObjects` _returnvalue (+ _returnvalue (* (`KismetMathLibrary.GetForwardVector` (`Pawn.GetBaseAimRotation` _aspawn)) 2000.0)) (`self.Object Types`) false (`|MakeArray` (`self.Placeable Preview Object`) :!type "Actor Object Reference")))
    (if _returnvalue_2
      (bind _returnvalue_3 (`|SpawnActorFromClass` (`self.SelectedDefense`) (`KismetMathLibrary.MakeTransform` (`SceneComponent.K2_GetComponentLocation` (`/Game/Sandboxes/Chadwick/BP_PlaceablePreview.Mesh` _placeable_preview_object)) (`Actor.K2_GetActorRotation` _placeable_preview_object)) "Undefined" "OverrideRootScale" null null))
      (`Actor.K2_AttachToComponent` _returnvalue_3 (`.HitComponent` (`GameplayStatics.BreakHitResult` _outhit)) "None" "KeepWorld" "KeepWorld" "KeepWorld" true)
      (`|SpawnActorFromClass` (`self.Builder Drone Class`) (`KismetMathLibrary.MakeTransform` (+ (`SceneComponent.K2_GetComponentLocation` (`/Game/Sandboxes/Chadwick/BP_PlaceablePreview.Mesh` (`self.Placeable Preview Object`))) (0.0 0.0 -10.0))) "AlwaysSpawn" "OverrideRootScale" null null)
      (`self.ChangeScrapCount` (* (`.Cost_21_365446DF4E58E68996D2948C11897BFE` (break `/Game/CyberSiege/Core/Widgets/FTielListEntryData` (`self.Selected Defense Data`))) -1))
      (bind _asteleporter (cast `Teleporter` _returnvalue_3))
      (`self.FindPartnerTeleporter` _asteleporter)
      (else
        (`KismetSystemLibrary.PrintString` "Invalid defense placement")))))

(fn `Rotate Placeable`
  (params (Axis :type "Float (double-precision)"))
  (if (and (!= Axis 0.0) (`self.Active`) (`KismetSystemLibrary.IsValid` (`self.Placeable Preview Object`)))
    (`Actor.K2_AddActorLocalRotation` (`self.Placeable Preview Object`) (`KismetMathLibrary.MakeRotator` 0.0 0.0 (* Axis (`self.Rotation Speed`))) false false)))

(fn `Scroll Wheel`
  (params (Axis :type "Float (double-precision)"))
  (switch `/Game/CyberSiege/Core/Actors/ActorComponents/EBuildStates` (`self.Build State`)
    (:`NewEnumerator0`
      (`self.OnScrollWheel` Axis :!label _label))
    (:`NewEnumerator1`
      (goto _label))
    (:`NewEnumerator2`
      (`self.Rotate Placeable` Axis))))

(fn `Set Selected Defense`
  (params (`New Defense` :type "/Game/CyberSiege/Core/Widgets/FTielListEntryData Structure"))
  (set `self.Selected Defense Data` `New Defense`)
  (set `self.SelectedDefense` (`.DefenseClass_20_D32611B3438D94434D5FCAB4CB169DEC` (break `/Game/CyberSiege/Core/Widgets/FTielListEntryData` `New Defense`))))

(fn `Update Build State`
  (params (`New State` :type "/Game/CyberSiege/Core/Actors/ActorComponents/EBuildStates Enum" :default "NewEnumerator0"))
  (set `self.Build State` `New State`))

(fn `Update Placeable Preview`
  (locals (`End Point` :type "Vector Structure"))
  (bind _dynamic_material (`self.Dynamic Material`))
  (bind _placeable_preview_object (`self.Placeable Preview Object`))
  (bind (_bounding_box_extents_x _bounding_box_extents_y _bounding_box_extents_z) (`KismetMathLibrary.BreakVector` (`self.Bounding Box Extents`)))
  (bind _returnvalue (`PlayerCameraManager.GetCameraLocation` (`GameplayStatics.GetPlayerCameraManager` 0)))
  (if (`|EnumEquality` (`self.Build State`) "NewEnumerator2")
    (bind _aspawn (cast `Pawn` (`self.GetOwner`)))
    (bind _output_get (set `local.End Point` (+ _returnvalue (* (`KismetMathLibrary.GetForwardVector` (`Pawn.GetBaseAimRotation` _aspawn)) 2000.0))))
    (bind (_outhit _returnvalue_2) (`KismetSystemLibrary.LineTraceSingleForObjects` _returnvalue _output_get (`self.Object Types`) false (`|MakeArray` (`self.Placeable Preview Object`) :!type "Actor Object Reference")))
    (bind _asturret_platform (cast `TurretPlatform` (`.HitActor` (`GameplayStatics.BreakHitResult` _outhit)))
      (:`then`
        (set `local.End Point` (`SceneComponent.GetSocketLocation` (`TurretPlatform.Mesh` _asturret_platform) (`self.PlatformSocketName`)))
        (bind _returnvalue_3 (+ (stale _output_get_2) (`KismetMathLibrary.MakeVector` 0.0 0.0 (+ _bounding_box_extents_z 10.0))))
        (bind (_outhit_2 _returnvalue_4) (`KismetSystemLibrary.BoxTraceSingleForObjects` _returnvalue_3 _returnvalue_3 (`KismetMathLibrary.MakeVector` _bounding_box_extents_x _bounding_box_extents_y _bounding_box_extents_z) (`Actor.K2_GetActorRotation` _placeable_preview_object) (`self.Area Detection Objects`) false (`|MakeArray` _placeable_preview_object :!type "Actor Object Reference") :!label _label))
        (if (or _returnvalue_4 (< (`self.ScrapCount`) (`.Cost_21_365446DF4E58E68996D2948C11897BFE` (break `/Game/CyberSiege/Core/Widgets/FTielListEntryData` (`self.Selected Defense Data`)))))
          (`MaterialInstanceDynamic.SetVectorParameterValue` _dynamic_material "Color" (struct :`R` 0.375 :`A` 0.75) :!label _label_2)
          (set `self.Placement Valid` false)
          (else
            (`MaterialInstanceDynamic.SetVectorParameterValue` _dynamic_material "Color" (struct :`G` 0.375 :`A` 0.75))
            (set `self.Placement Valid` true))))
      (:`CastFailed`
        (if _returnvalue_2
          (bind _output_get_2 (set `local.End Point` (`.ImpactPoint` (`GameplayStatics.BreakHitResult` _outhit))))
          (goto _label)
          (else
            (goto _label_2)))))
    (`SceneComponent.K2_SetWorldLocation` (`/Game/Sandboxes/Chadwick/BP_PlaceablePreview.Mesh` (`self.Placeable Preview Object`)) (`local.End Point`) false false)))