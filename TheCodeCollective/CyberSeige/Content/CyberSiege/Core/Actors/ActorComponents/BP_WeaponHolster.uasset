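; BP_WeaponHolster is an actor component that manages primary and secondary weapon slots and throwable ammo.
; New weapons fill an empty slot or destroy and replace the held one; switching toggles or selects a slot, and is blocked mid-throw.
; Throws temporarily swap in a spawned BP_Unarmed, restoring the previous weapon when the animation ends.
; Dispatchers broadcast throwable use and ammo changes; a looping timer starts at BeginPlay alongside a grenade-replenish event.
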(event `self.ReceiveBeginPlay`
  (bind _max_throwble_ammo (`self.Max Throwble Ammo`))
  ;[1 1 1] In Code
  (bind _output_get (set `self.Current Throwble Ammo` _max_throwble_ammo))
  (`self.OnThrowableAmmoChanged` _output_get _max_throwble_ammo)
  (`KismetSystemLibrary.K2_SetTimerDelegate` (`|CreateDelegate` :!event `Replenish Grenade`) 20.0 true))

(event `Replace Weapon`
  (params (`New Weapon` :type "/Game/CyberSiege/Core/Actors/Weapons/BP_BaseWeapon Object Reference"))
  (bind _currentweapon (`self.CurrentWeapon`))
  (if (`KismetSystemLibrary.IsValid` `New Weapon`)
    (if (or (not (`KismetSystemLibrary.IsValid` (`self.Primary`))) (not (`KismetSystemLibrary.IsValid` (`self.Secondary`))))
      (if (`KismetSystemLibrary.IsValid` (`self.Primary`))
        (if (not (`KismetSystemLibrary.IsValid` (`self.Secondary`)))
          (bind _output_get (set `self.Secondary` `New Weapon`))
          (set `self.CurrentWeapon` _output_get))
        (else
          (bind _output_get_2 (set `self.Primary` `New Weapon`))
          (set `self.CurrentWeapon` _output_get_2)))
      (elif (`KismetSystemLibrary.IsValid` (`self.CurrentWeapon`))
        (if (== (`self.Primary`) _currentweapon)
          (`Actor.K2_DestroyActor` (`self.Primary`))
          (bind _output_get_3 (set `self.Primary` `New Weapon`))
          (set `self.CurrentWeapon` _output_get_3)
          (elif (== _currentweapon (`self.Secondary`))
            (`Actor.K2_DestroyActor` (`self.Secondary`))
            (bind _output_get_4 (set `self.Secondary` `New Weapon`))
            (set `self.CurrentWeapon` _output_get_4)))))))

(event `Replenish Grenade`
  (if (< (`self.Current Throwble Ammo`) (`self.Max Throwble Ammo`))
    (bind _result (`/Engine/EditorBlueprintResources/StandardMacros.IncrementInt` (`self.Current Throwble Ammo`))
      (:`  `
        (`self.OnThrowableAmmoChanged` _result (`self.Max Throwble Ammo`))))))

(event `Goto Weapon`
  (params (`New Weapon` :type Integer))
  (if (not (`self.Throwing Grenade`))
    (switch `int` `New Weapon`
      (:`Default`
        (`KismetSystemLibrary.PrintString` "ERROR: Invalid integer provided for \"Weapon Override\" in WeaponHolser"))
      (:`0`
        (`self.Change Current Weapon` (`self.Primary`)))
      (:`1`
        (`self.Change Current Weapon` (`self.Secondary`))))))

(event `Switch Weapon`
  (if (not (`self.Throwing Grenade`))
    (`self.Change Current Weapon` null)))

(fn `Can Use Throwable`
  (returns (Boolean :type Boolean))
  (return (and (> (`self.Current Throwble Ammo`) 0) (not (`self.Throwing Grenade`)))))

(fn `Change Current Weapon`
  (params (`Weapon Override` :type "/Game/CyberSiege/Core/Actors/Weapons/BP_BaseWeapon Object Reference"))
  (if (`KismetSystemLibrary.IsValid` `Weapon Override`)
    (set `self.CurrentWeapon` (`local.Weapon Override`))
    (elif (`KismetSystemLibrary.IsValid` (`self.CurrentWeapon`))
      (if (== (`self.CurrentWeapon`) (`self.Primary`))
        (if (`KismetSystemLibrary.IsValid` (`self.Secondary`))
          (set `self.CurrentWeapon` (`self.Secondary`)))
        (elif (`KismetSystemLibrary.IsValid` (`self.Primary`))
          (set `self.CurrentWeapon` (`self.Primary`))))
      (elif (`KismetSystemLibrary.IsValid` (`self.Primary`))
        (set `self.CurrentWeapon` (`self.Primary`))
        (elif (`KismetSystemLibrary.IsValid` (`self.Secondary`))
          (set `self.CurrentWeapon` (`self.Secondary`)))))))

(fn `Play Throwable Animation`
  (set `self.Throwing Grenade` true)
  (bind _returnvalue (`|SpawnActorFromClass` "/Game/CyberSiege/Core/Actors/Weapons/BP_Unarmed.BP_Unarmed_C" (`KismetMathLibrary.MakeTransform` (0.0 0.0 0.0)) "Undefined" "OverrideRootScale" null null))
  (set `self.Temp Weapon` (`self.CurrentWeapon`))
  (`self.Change Current Weapon` _returnvalue)
  (`self.OnThrowableUsed` (`self.Throwable Animation`))
  (bind _result (`/Engine/EditorBlueprintResources/StandardMacros.DecrementInt` (`self.Current Throwble Ammo`))
    (:`  `
      (bind _output_get (set `self.Current Throwble Ammo` _result))
      (`self.OnThrowableAmmoChanged` _output_get (`self.Max Throwble Ammo`)))))

(fn `Throwable Animation Ended`
  (`Actor.K2_DestroyActor` (`self.CurrentWeapon`))
  (`self.Change Current Weapon` (`self.Temp Weapon`))
  (set `self.Throwing Grenade` false))