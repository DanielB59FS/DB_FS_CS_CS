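; Drone enemy that lasers the castle, turrets and other blackboard targets.
; Attack turns the mesh toward the target and line-traces, damaging close non-Enemy hits while toggling beam and sound and leaving burn decals.
; Die ragdolls the drone, awards score, and drops either a rare health pickup or scrap plus a possible LaserFence quest trigger.
; Timed delays then damp its velocity before destroying it and its drop.
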(event `self.ReceiveBeginPlay`
  (`parent.ReceiveBeginPlay`)
  (`PrimitiveComponent.SetCollisionEnabled` (`self.LeftHandCollision`) "NoCollision")
  (`PrimitiveComponent.SetCollisionEnabled` (`self.RightHandCollision`) "NoCollision")
  (`SceneComponent.SetVisibility` (`self.LaserBeam`) false false))

(event `/Game/CyberSiege/Core/Interfaces/BPI_Enemies.UpdateAnimations`)

(event `self.Die`
  (params (HealthRatio :type "Float (single-precision)"))
  (bind _mesh (`self.Mesh`))
  (bind _lasersound (`self.LaserSound`))
  (bind _mesh_2 (`self.Mesh`))
  (bind _mapmarker (`self.MapMarker`))
  (bind _mesh_3 (`self.Mesh`))
  (bind (_returnvalue_x _returnvalue_y _returnvalue_z) (`KismetMathLibrary.BreakVector` (`SceneComponent.K2_GetComponentLocation` (`self.Mesh`))))
  (set `self.IsDead` true)
  (`PrimitiveComponent.SetPhysicsLinearVelocity` (`self.CapsuleComponent`) (0.0 0.0 0.0) false "None")
  (`PrimitiveComponent.SetSimulatePhysics` (`self.Mesh`) true)
  (`PrimitiveComponent.SetCollisionResponseToChannel` (`self.CapsuleComponent`) "ECC_GameTraceChannel1" "ECR_Ignore")
  (`PrimitiveComponent.SetCollisionResponseToChannel` _mesh_2 "ECC_GameTraceChannel1" "ECR_Ignore")
  (`PrimitiveComponent.SetCollisionObjectType` _mesh_2 "ECC_PhysicsBody")
  (`PrimitiveComponent.SetCollisionObjectType` (`self.CapsuleComponent`) "ECC_PhysicsBody")
  (if (>= (`KismetMathLibrary.RandomInteger` (`self.RandomMax`)) 95)
    (bind _returnvalue (`|SpawnActorFromClass` "/Game/CyberSiege/Core/Actors/BP_HealthPickup.BP_HealthPickup_C" (`KismetMathLibrary.MakeTransform` (`KismetMathLibrary.MakeVector` _returnvalue_x _returnvalue_y (- _returnvalue_z 200.0)) (struct) (2.0 2.0 2.0)) "AlwaysSpawn" "OverrideRootScale" self null))
    (bind _output_get (set `self.HealthPickup` _returnvalue))
    (`self.K2_AttachToActor` _output_get self "HealthPickupSocket" "KeepWorld" "KeepWorld" "KeepRelative" false)
    (else
      (bind _returnvalue_2 (`|SpawnActorFromClass` "/Game/CyberSiege/Core/Actors/Spawners/BP_ScrapSpawner.BP_ScrapSpawner_C" (`self.GetTransform` self) "AdjustIfPossibleButAlwaysSpawn" "OverrideRootScale" self null))
      ;[1 1 1] Quest trigger spawning
      (`self.SpawnQuestTrigger`)
      (bind _output_get_2 (set `self.ScrapSpawner` _returnvalue_2))
      (`BaseScrap.SetScrapAmount` _output_get_2 10.0)
      (`self.K2_AttachToComponent` _output_get_2 (`self.Mesh`) "ScrapSpawnerSocket" "SnapToTarget" "KeepRelative" "KeepRelative" true)))
  (`SceneComponent.SetVisibility` (`self.LaserBeam`) false false)
  (if (!= _lasersound null)
    (if (`AudioComponent.IsPlaying` _lasersound)
      (`AudioComponent.Stop` _lasersound)))
  (`self.OnEnemyDied`)
  ;[1 1 1] temp
  (`/Game/CyberSiege/Core/Engine/BP_GameInstance.AddScore` (cast `/Game/CyberSiege/Core/Engine/BP_GameInstance` (`GameplayStatics.GetGameInstance`) :!pure true) self "NewEnumerator3")
  (`KismetMathLibrary.LinearColor_Set` (`/Game/CyberSiege/Core/Widgets/Minimap/BP_MapMarkerComponent.MarkerColor` _mapmarker) (struct :`A` 0.5))
  (`/Game/CyberSiege/Core/Widgets/Minimap/BP_MapMarkerComponent.UpdateMarkerProperties` _mapmarker)
  (`KismetSystemLibrary.Delay` 1.5)
  (bind _returnvalue_3 (`PrimitiveComponent.GetPhysicsLinearVelocity` _mesh_3 "None"))
  (`PrimitiveComponent.SetPhysicsLinearVelocity` _mesh_3 (/ _returnvalue_3 2.0) false "None")
  (`PrimitiveComponent.SetAllPhysicsAngularVelocityInDegrees` _mesh_3 (/ (`PrimitiveComponent.GetPhysicsAngularVelocityInDegrees` _mesh_3 "None") 2.0) false)
  (`KismetSystemLibrary.Delay` 0.5)
  (`PrimitiveComponent.SetPhysicsLinearVelocity` _mesh (0.0 0.0 0.0) false "None")
  (`PrimitiveComponent.SetAllPhysicsAngularVelocityInDegrees` _mesh (`self.ZeroAngVel`) false)
  (`PrimitiveComponent.SetCollisionEnabled` (`self.CapsuleComponent`) "NoCollision")
  (`KismetSystemLibrary.Delay` (`self.TimeUntilDestroy`))
  (`self.K2_DestroyActor`)
  (if (!= (`self.ScrapSpawner`) null)
    (`self.K2_DestroyActor` (`self.ScrapSpawner`))
    (elif (!= (`self.HealthPickup`) null)
      (`self.K2_DestroyActor` (`self.HealthPickup`)))))

(event `/Game/CyberSiege/Core/Interfaces/BPI_Enemies.Attack`
  (params (ControlledPawn :type "Object Object Reference"))
  (bind _returnvalue (`self.GetInstigatorController`))
  (bind _lasersound (`self.LaserSound`))
  (bind _laserbeam (`self.LaserBeam`))
  (bind _laserbeam_2 (`self.LaserBeam`))
  (bind _returnvalue_2 (`SceneComponent.K2_GetComponentLocation` (`self.Mesh`)))
  (bind _resultlocation (`BlackboardComponent.GetLocationFromEntry` (`self.Blackboard`) (`self.BBCurrentTargetKeyName`)))
  (bind (_returnvalue_roll _returnvalue_pitch _returnvalue_yaw) (`KismetMathLibrary.BreakRotator` (`KismetMathLibrary.FindLookAtRotation` _returnvalue_2 _resultlocation)))
  (bind _y (.y (`BlackboardComponent.GetValueAsVector` (`self.Blackboard`) (`self.BBCastleLocationKeyName`))))
  (bind _z (.z (`BlackboardComponent.GetValueAsVector` (`self.Blackboard`) (`self.BBCastleLocationKeyName`))))
  (bind _returnvalue_3 (- (.x (`BlackboardComponent.GetValueAsVector` (`self.Blackboard`) (`self.BBCastleLocationKeyName`))) 100.0))
  (bind (_returnvalue_roll_2 _returnvalue_pitch_2 _returnvalue_yaw_2) (`KismetMathLibrary.BreakRotator` (`KismetMathLibrary.FindLookAtRotation` _returnvalue_2 (`KismetMathLibrary.MakeVector` _returnvalue_3 _y _z))))
  (if (not (`self.IsDead`))
    (if (== _resultlocation (`self.K2_GetActorLocation` (`self.Castle`)))
      (bind _result (`/Engine/EditorBlueprintResources/StandardMacros.NegateFloat` _returnvalue_pitch_2)
        (:`  `
          (bind (_outhit _hitsomething) (`self.RotateAndLineTrace` (`KismetMathLibrary.MakeVector` _returnvalue_3 _y _z) _result _returnvalue_roll_2 (- _returnvalue_yaw_2 90.0)))
          (if _hitsomething
            (bind (_bblockinghit _binitialoverlap _time _distance _location _impactpoint _normal _impactnormal _physmat _hitactor) (`GameplayStatics.BreakHitResult` _outhit))
            (if (< _distance 500.0)
              (`GameplayStatics.SpawnDecalAtLocation` "/Game/AssetMigration/Materials/charcoal-Unreal-Engine/M_Burn.M_Burn" (50.0 50.0 50.0) _location (`KismetMathLibrary.Conv_VectorToRotator` _impactnormal) 30.0))
            (bind (_distancebool __containsenemy _containscastle) (`self.LessThanAndContains` _distance _hitactor))
            (if _distancebool
              (if __containsenemy
                (if _containscastle
                  ;[1 1 1] castle
                  (`GameplayStatics.ApplyDamage` (`self.Castle`) (`self.Base Damage`) _returnvalue self :!label _label)
                  (else
                    (`GameplayStatics.ApplyDamage` _hitactor (`self.Base Damage`) _returnvalue self)))
                (`SceneComponent.SetVisibility` _laserbeam true false :!label _label_2)
                (`/Engine/EditorBlueprintResources/StandardMacros.DoOnce` false :!label _label_3
                  (:`Completed`
                    (bind _returnvalue_4 (`GameplayStatics.SpawnSoundAttached` "/Game/CyberSiege/Audio/SFX/AI/A_DroneEnemyAttackSound.A_DroneEnemyAttackSound" _laserbeam_2 "None" (`SceneComponent.K2_GetComponentLocation` _laserbeam_2) (struct) "SnapToTargetIncludingScale" true 0.15 1.0 0.0 null null false))
                    (set `self.LaserSound` _returnvalue_4)))
                (else
                  (`SceneComponent.SetVisibility` (`self.LaserBeam`) false false :!label _label_4)
                  (if (!= (`self.LaserSound`) null)
                    (`AudioComponent.Stop` (`self.LaserSound`))
                    (goto _label_3 :!via `Reset`))))
              (else
                (goto _label_4)))
            (else
              (goto _label_4)))))
      (else
        (bind _result_2 (`/Engine/EditorBlueprintResources/StandardMacros.NegateFloat` _returnvalue_pitch)
          (:`  `
            (bind (_outhit_2 _hitsomething_2) (`self.RotateAndLineTrace` _resultlocation _result_2 _returnvalue_roll (- _returnvalue_yaw 90.0)))
            (if _hitsomething_2
              (bind (_bblockinghit_2 _binitialoverlap_2 _time_2 _distance_2 _location_2 _impactpoint_2 _normal_2 _impactnormal_2 _physmat_2 _hitactor_2) (`GameplayStatics.BreakHitResult` _outhit_2))
              (if (< _distance_2 500.0)
                (`GameplayStatics.SpawnDecalAtLocation` "/Game/AssetMigration/Materials/charcoal-Unreal-Engine/M_Burn.M_Burn" (50.0 50.0 50.0) _location_2 (`KismetMathLibrary.Conv_VectorToRotator` _impactnormal_2) 30.0))
              (bind (_distancebool_2 __containsenemy_2 _containscastle_2) (`self.LessThanAndContains` _distance_2 _hitactor_2))
              (if _distancebool_2
                (if __containsenemy_2
                  (if _containscastle_2
                    (goto _label)
                    (else
                      (`GameplayStatics.ApplyDamage` _hitactor_2 (`self.Base Damage`) _returnvalue self)
                      (if (`KismetSystemLibrary.IsValid` _hitactor_2)
                        (bind _returnvalue_5 (`GameplayStatics.GetObjectClass` _hitactor_2))
                        (if (== _returnvalue_5 "/Game/CyberSiege/Core/Actors/Defenses/BP_BaseTurret.BP_BaseTurret_C")
                          (bind _asbp_base_turret (cast `/Game/CyberSiege/Core/Actors/Defenses/BP_BaseTurret` _hitactor_2))
                          (if (<= (`/Game/CyberSiege/Core/Actors/ActorComponents/BP_HealthComponent.CurrentHealth` (`/Game/CyberSiege/Core/Actors/Defenses/BP_BaseTurret.BP_HealthComponent` _asbp_base_turret)) 0.0)
                            _
                            (else
                              (goto _label_2)))
                          (elif (== _returnvalue_5 "/Game/CyberSiege/Core/Actors/Defenses/BP_GrenadeTurret.BP_GrenadeTurret_C")
                            (bind _asbp_grenade_turret (cast `/Game/CyberSiege/Core/Actors/Defenses/BP_GrenadeTurret` _hitactor_2))
                            (if (<= (`/Game/CyberSiege/Core/Actors/ActorComponents/BP_HealthComponent.CurrentHealth` (`/Game/CyberSiege/Core/Actors/Defenses/BP_GrenadeTurret.BP_HealthComponent` _asbp_grenade_turret)) 0.0)
                              _
                              (else
                                (goto _label_2)))
                            (elif (== _returnvalue_5 "/Game/CyberSiege/Core/Actors/Defenses/BP_SniperTurret.BP_SniperTurret_C")
                              (bind _asbp_sniper_turret (cast `/Game/CyberSiege/Core/Actors/Defenses/BP_SniperTurret` _hitactor_2))
                              (if (<= (`/Game/CyberSiege/Core/Actors/ActorComponents/BP_HealthComponent.CurrentHealth` (`/Game/CyberSiege/Core/Actors/Defenses/BP_SniperTurret.BP_HealthComponent` _asbp_sniper_turret)) 0.0)
                                _
                                (else
                                  (goto _label_2)))
                              (else
                                (goto _label_2))))))
                      (`SceneComponent.SetVisibility` _laserbeam false false)
                      (if (`KismetSystemLibrary.IsValid` _lasersound)
                        (`AudioComponent.Stop` _lasersound)
                        (goto _label_3 :!via `Reset`))))
                  (else
                    (goto _label_4)))
                (else
                  (goto _label_4)))
              (else
                (goto _label_4)))))))))

(event `/Game/CyberSiege/Core/Interfaces/BPI_Enemies.DroneLaserOff`
  (bind _lasersound (`self.LaserSound`))
  (`SceneComponent.SetVisibility` (`self.LaserBeam`) false false)
  (if (`KismetSystemLibrary.IsValid` _lasersound)
    (`AudioComponent.Stop` _lasersound)))

(fn `LessThanAndContains`
  (params (Distance :type "Float (double-precision)") (HitActor :type "Actor Object Reference"))
  (returns (DistanceBool :type Boolean) (`!ContainsEnemy` :type Boolean) (ContainsCastle :type Boolean))
  (bind _tags (`Actor.Tags` HitActor))
  (return (< Distance 500.0) (not (`KismetArrayLibrary.Array_Contains` _tags "Enemy")) (`KismetArrayLibrary.Array_Contains` _tags "Castle")))

(fn `RotateAndLineTrace`
  (params (AttackLocation :type "Vector Structure") (RotationX :type "Float (double-precision)") (RotationY :type "Float (double-precision)") (RotationZ :type "Float (double-precision)"))
  (returns (OutHit :type "HitResult Structure") (HitSomething :type Boolean))
  (bind _mesh (`self.Mesh`))
  (`SceneComponent.K2_SetWorldRotation` _mesh (`KismetMathLibrary.MakeRotator` RotationX RotationY RotationZ) false false)
  (bind (_outhit _returnvalue) (`KismetSystemLibrary.LineTraceSingleForObjects` :`Start` (`SceneComponent.K2_GetComponentLocation` _mesh) :`End` AttackLocation :`ObjectTypes` (`self.Object Types`) :`DrawTime` 2.0))
  (return _outhit _returnvalue))

(fn `SpawnQuestTrigger`
  ;[1 1 1] Very quick and dirty way to spawn a quest trigger for the laser fence quest
  (bind _returnvalue (`GameplayStatics.GetActorOfClass` "/Game/CyberSiege/Core/Actors/Quest/BP_QuestManager.BP_QuestManager_C"))
  (bind (_questkey _questcompletemessage _queststeps _activestep) (break `Quest` (`QuestManager.ActiveQuest` _returnvalue)))
  (bind (_queststeptext _triggers _activators _binitialstep _bfinalstep _bskipifnotriggers _bismultitrigger _busesindicator _dialoguetext _boundtriggercount _triggersneeded) (break `QuestStep` _activestep))
  (if (and (`KismetStringLibrary.EqualEqual_StrStr` _questkey "LaserFence") (== _triggersneeded 5) (< _boundtriggercount 5))
    (`|SpawnActorFromClass` "/Game/CyberSiege/Core/Actors/Quest/BP_QuestPlayerTrigger_Physics.BP_QuestPlayerTrigger_Physics_C" (`self.GetTransform`) "Undefined" "OverrideRootScale" null (`self.GetInstigator`))))

(fn `UserConstructionScript`
  (`parent.UserConstructionScript`))