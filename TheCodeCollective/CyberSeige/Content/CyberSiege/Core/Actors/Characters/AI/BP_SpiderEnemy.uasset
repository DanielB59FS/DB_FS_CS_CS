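; Spider enemy AI character that shoots at targets, including the castle, and drops loot on death.
; Movement, attack and death drive ABP_SpiderEnemy through speed, direction and a state enum.
; Attack line-traces from the muzzle socket to the blackboard target, damaging close non-enemy hits and redirecting Castle-tagged hits to the Castle reference.
; Death unpossesses, ragdolls if airborne, randomly drops health or scrap, awards score, then destroys itself and the drop after a delay.
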(event `self.ReceiveBeginPlay`
  (`parent.ReceiveBeginPlay`)
  (`PrimitiveComponent.SetCollisionEnabled` (`self.LeftHandCollision`) "NoCollision")
  (`PrimitiveComponent.SetCollisionEnabled` (`self.RightHandCollision`) "NoCollision"))

(event `self.ReceiveTick`
  (params (DeltaSeconds :type "Float (single-precision)"))
  (`parent.ReceiveTick` DeltaSeconds)
  (bind _asabp_spider_enemy (cast `/Game/CyberSiege/Core/Animations/Characters/AI/ABP_SpiderEnemy` (`SkeletalMeshComponent.GetAnimInstance` (`self.Mesh`)))
    (:`then`
      (if (> (`/Game/CyberSiege/Core/Animations/Characters/AI/ABP_SpiderEnemy.Speed` _asabp_spider_enemy) 1.0)
        (set `/Game/CyberSiege/Core/Animations/Characters/AI/ABP_SpiderEnemy.Enum` "NewEnumerator0" _asabp_spider_enemy)))
    (:`CastFailed`
      (`KismetSystemLibrary.PrintString` "spider animation not ABP_SpiderEnemy (spider enemy tick)"))))

(event `/Game/CyberSiege/Core/Interfaces/BPI_Enemies.UpdateAnimations`
  (bind _returnvalue (`self.GetVelocity`))
  (bind _asabp_spider_enemy (cast `/Game/CyberSiege/Core/Animations/Characters/AI/ABP_SpiderEnemy` (`SkeletalMeshComponent.GetAnimInstance` (`self.Mesh`)))
    (:`then`
      (set `/Game/CyberSiege/Core/Animations/Characters/AI/ABP_SpiderEnemy.Speed` (`KismetMathLibrary.VSize` _returnvalue) _asabp_spider_enemy)
      (set `/Game/CyberSiege/Core/Animations/Characters/AI/ABP_SpiderEnemy.Direction` (`AnimInstance.CalculateDirection` _asabp_spider_enemy _returnvalue (`self.K2_GetActorRotation`)) _asabp_spider_enemy))
    (:`CastFailed`
      (`KismetSystemLibrary.PrintString` "Could not cast anim instance to ABP_SpiderEnemy (BP_SpiderEnemy)"))))

(event `/Game/CyberSiege/Core/Interfaces/BPI_Enemies.Attack`
  (params (ControlledPawn :type "Object Object Reference"))
  (bind _returnvalue (`self.GetInstigatorController`))
  (bind _mesh (`self.Mesh`))
  (bind _returnvalue_2 (`SceneComponent.GetSocketLocation` _mesh "MuzzleFlashSocket"))
  (if (not (`self.IsDead`))
    (bind _asabp_spider_enemy (cast `/Game/CyberSiege/Core/Animations/Characters/AI/ABP_SpiderEnemy` (`SkeletalMeshComponent.GetAnimInstance` (`self.Mesh`)))
      (:`then`
        (set `/Game/CyberSiege/Core/Animations/Characters/AI/ABP_SpiderEnemy.Enum` "NewEnumerator1" _asabp_spider_enemy)
        (`GameplayStatics.SpawnEmitterAtLocation` "/Game/AssetMigration/MilitaryWeapSilver/FX/P_Pistol_MuzzleFlash_01.P_Pistol_MuzzleFlash_01" _returnvalue_2 (`SceneComponent.K2_GetComponentRotation` _mesh))
        (`GameplayStatics.SpawnSoundAtLocation` "/Game/CyberSiege/Audio/SFX/AI/A_SpiderEnemyAttackSound.A_SpiderEnemyAttackSound" _returnvalue_2 (struct) 0.15 0.9 0.0 null null)
        (bind (_outhit _returnvalue_3) (`KismetSystemLibrary.LineTraceSingleForObjects` :`Start` (`SceneComponent.GetSocketLocation` (`self.Mesh`) "MuzzleFlashSocket") :`End` (`BlackboardComponent.GetLocationFromEntry` (`self.Blackboard`) (`self.BBCurrentTargetKeyName`)) :`ObjectTypes` (`self.Object Types`) :`DrawTime` 2.0))
        (if _returnvalue_3
          (bind (_bblockinghit _binitialoverlap _time _distance _location _impactpoint _normal _impactnormal _physmat _hitactor) (`GameplayStatics.BreakHitResult` _outhit))
          (bind _tags (`Actor.Tags` _hitactor))
          (if (and (not (`KismetArrayLibrary.Array_Contains` _tags "Enemy")) (< _distance 500.0))
            (if (`KismetArrayLibrary.Array_Contains` _tags "Castle")
              (`GameplayStatics.ApplyDamage` (`self.Castle`) 0.25 _returnvalue self)
              (else
                (`GameplayStatics.ApplyDamage` _hitactor 0.25 _returnvalue self))))))
      (:`CastFailed`
        (`KismetSystemLibrary.PrintString` "not ABP_SpiderEnemy (SpiderEnemy)")))))

(event `self.Die`
  (params (HealthRatio :type "Float (single-precision)"))
  (bind (_returnvalue_location _returnvalue_rotation) (`KismetMathLibrary.BreakTransform` (`self.GetTransform`)))
  (bind _mapmarker (`self.MapMarker`))
  (set `self.IsDead` true)
  (bind _asabp_spider_enemy (cast `/Game/CyberSiege/Core/Animations/Characters/AI/ABP_SpiderEnemy` (`SkeletalMeshComponent.GetAnimInstance` (`self.Mesh`)))
    (:`then`
      (set `/Game/CyberSiege/Core/Animations/Characters/AI/ABP_SpiderEnemy.Enum` "NewEnumerator2" _asabp_spider_enemy)
      (if (`NavMovementComponent.IsMovingOnGround` (`self.CharacterMovement`))
        (`MovementComponent.StopMovementImmediately` (`self.CharacterMovement`))
        (else
          (`MovementComponent.StopMovementImmediately` (`self.CharacterMovement`))
          (`PrimitiveComponent.SetSimulatePhysics` (`self.Mesh`) true)))
      (`Controller.UnPossess` (`AIBlueprintHelperLibrary.GetAIController` self))
      (`PrimitiveComponent.SetCollisionEnabled` (`self.CapsuleComponent`) "NoCollision")
      (if (>= (`KismetMathLibrary.RandomInteger` (`self.RandomMax`)) 95)
        (bind _returnvalue (`|SpawnActorFromClass` "/Game/CyberSiege/Core/Actors/BP_HealthPickup.BP_HealthPickup_C" (`KismetMathLibrary.MakeTransform` _returnvalue_location _returnvalue_rotation (2.0 2.0 2.0)) "AlwaysSpawn" "OverrideRootScale" self null))
        (bind _output_get (set `self.HealthPickup` _returnvalue))
        (`self.K2_AttachToComponent` _output_get (`self.Mesh`) "None" "KeepWorld" "KeepRelative" "KeepRelative" true)
        (else
          (bind _returnvalue_2 (`|SpawnActorFromClass` "/Game/CyberSiege/Core/Actors/Spawners/BP_ScrapSpawner.BP_ScrapSpawner_C" (`self.GetTransform` self) "AlwaysSpawn" "OverrideRootScale" self null))
          (bind _output_get_2 (set `self.ScrapSpawner` _returnvalue_2))
          (`BaseScrap.SetScrapAmount` _output_get_2 10.0)
          (`self.K2_AttachToComponent` _output_get_2 (`self.Mesh`) "None" "KeepWorld" "KeepRelative" "KeepRelative" true)))
      (`self.OnEnemyDied`)
      ;[1 1 1] temp
      (`/Game/CyberSiege/Core/Engine/BP_GameInstance.AddScore` (cast `/Game/CyberSiege/Core/Engine/BP_GameInstance` (`GameplayStatics.GetGameInstance`) :!pure true) self "NewEnumerator3")
      (`KismetMathLibrary.LinearColor_Set` (`/Game/CyberSiege/Core/Widgets/Minimap/BP_MapMarkerComponent.MarkerColor` _mapmarker) (struct :`A` 0.5))
      (`/Game/CyberSiege/Core/Widgets/Minimap/BP_MapMarkerComponent.UpdateMarkerProperties` _mapmarker)
      (`KismetSystemLibrary.Delay` (`self.TimeUntilDestroy`))
      (`self.K2_DestroyActor`)
      (if (!= (`self.ScrapSpawner`) null)
        (`self.K2_DestroyActor` (`self.ScrapSpawner`))
        (elif (!= (`self.HealthPickup`) null)
          (`self.K2_DestroyActor` (`self.HealthPickup`)))))
    (:`CastFailed`
      (`KismetSystemLibrary.PrintString` "not ABP_spiderEnemy (spider enemy)"))))

(fn `UserConstructionScript`
  (`SceneComponent.K2_AttachToComponent` (`self.HeadCollision`) (`self.Mesh`) "body" "KeepRelative" "KeepRelative" "KeepRelative" true))