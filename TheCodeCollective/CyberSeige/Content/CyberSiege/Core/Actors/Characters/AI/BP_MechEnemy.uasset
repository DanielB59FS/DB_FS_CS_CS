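; Mech enemy for a castle siege game, a heavier AI enemy worth double the parent's points.
; Attack reads the blackboard target, stomping nearby non-castle targets to damage non-enemies in StompBox, otherwise firing its child-actor shotgun via short line trace.
; Attack and death states drive ABP_MechEnemy through an enum, alongside speed, direction and a shotgun left-hand socket lookup.
; Death unpossesses it, spawns attached scrap, awards score, updates the map marker and destroys it after a delay.
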(event `self.ReceiveBeginPlay`
  (`parent.ReceiveBeginPlay`)
  (`PrimitiveComponent.SetCollisionEnabled` (`self.LeftHandCollision`) "NoCollision")
  (`PrimitiveComponent.SetCollisionEnabled` (`self.RightHandCollision`) "NoCollision"))

(event `/Game/CyberSiege/Core/Interfaces/BPI_Enemies.UpdateAnimations`
  (bind _returnvalue (`self.GetVelocity`))
  (bind _asabp_mech_enemy (cast `/Game/CyberSiege/Core/Animations/Characters/AI/ABP_MechEnemy` (`SkeletalMeshComponent.GetAnimInstance` (`self.Mesh`)))
    (:`then`
      (set `/Game/CyberSiege/Core/Animations/Characters/AI/ABP_MechEnemy.Speed` (`KismetMathLibrary.VSize` _returnvalue) _asabp_mech_enemy)
      (set `/Game/CyberSiege/Core/Animations/Characters/AI/ABP_MechEnemy.Direction` (`AnimInstance.CalculateDirection` _asabp_mech_enemy _returnvalue (`self.K2_GetActorRotation`)) _asabp_mech_enemy))
    (:`CastFailed`
      (`KismetSystemLibrary.PrintString` "Could not cast anim instance to ABP_MechEnemy (BP_MechEnemy)"))))

(event `/Game/CyberSiege/Core/Interfaces/BPI_Enemies.Attack`
  (params (ControlledPawn :type "Object Object Reference"))
  (bind _bbcurrenttargetkeyname (`self.BBCurrentTargetKeyName`))
  (bind _blackboard (`self.Blackboard`))
  (bind _object_types (`self.Object Types`))
  (bind _bbcurrenttargetkeyname_2 (`self.BBCurrentTargetKeyName`))
  (bind _blackboard_2 (`self.Blackboard`))
  (bind _p_impact_stone_large_01 (`self.P_Impact_Stone_Large_01`))
  (if (`self.CanDoDamage`)
    (bind _asabp_mech_enemy (cast `/Game/CyberSiege/Core/Animations/Characters/AI/ABP_MechEnemy` (`SkeletalMeshComponent.GetAnimInstance` (`self.Mesh`)))
      (:`then`
        (set `self.CanDoDamage` false)
        (if (!= (`BlackboardComponent.GetValueAsObject` _blackboard_2 _bbcurrenttargetkeyname_2) (`self.Castle`))
          (bind _outhit (`KismetSystemLibrary.LineTraceSingleForObjects` (`SceneComponent.K2_GetComponentLocation` (`self.Mesh`)) (`BlackboardComponent.GetLocationFromEntry` _blackboard_2 _bbcurrenttargetkeyname_2) (`self.Object Types`)))
          (if (< (`.Distance` (`GameplayStatics.BreakHitResult` _outhit)) 300.0)
            (`CharacterMovementComponent.DisableMovement` (`self.CharacterMovement`))
            ;[1 1 1] Stomp
            (set `/Game/CyberSiege/Core/Animations/Characters/AI/ABP_MechEnemy.MechEnum` "NewEnumerator4" _asabp_mech_enemy)
            (`KismetSystemLibrary.Delay` 0.74)
            (`GameplayStatics.SpawnEmitterAtLocation` "/Game/AssetMigration/MilitaryWeapSilver/FX/P_Impact_Stone_Large_01.P_Impact_Stone_Large_01" (`SceneComponent.K2_GetComponentLocation` _p_impact_stone_large_01) (`SceneComponent.K2_GetComponentRotation` _p_impact_stone_large_01))
            (for _array_element (`self.ActorsInStompBox`)
              (`GameplayStatics.ApplyDamage` _array_element (`self.BaseDamageMech`) (`AIBlueprintHelperLibrary.GetAIController` self) self))
            (`KismetSystemLibrary.Delay` 1.13)
            (set `self.CanDoDamage` true)
            (set `/Game/CyberSiege/Core/Animations/Characters/AI/ABP_MechEnemy.MechEnum` "NewEnumerator0" _asabp_mech_enemy)
            (`CharacterMovementComponent.SetMovementMode` (`self.CharacterMovement`) "MOVE_Walking" 0)
            (else
              (bind _asbp_aishotgun (cast `/Game/CyberSiege/Core/Actors/Weapons/AI/BP_AIShotgun` (`ChildActorComponent.ChildActor` (`self.ChildActorComponent`)) :!label _label)
                (:`then`
                  (bind _returnvalue (`SceneComponent.GetSocketLocation` (`/Game/CyberSiege/Core/Actors/Weapons/BP_BaseWeapon.Mesh` _asbp_aishotgun) "MuzzleSocket"))
                  (`GameplayStatics.SpawnEmitterAtLocation` "/Game/AssetMigration/MilitaryWeapSilver/FX/P_Shotgun_MuzzleFlash_01.P_Shotgun_MuzzleFlash_01" _returnvalue (`self.K2_GetActorRotation`) (2.5 2.5 2.5))
                  (`GameplayStatics.PlaySoundAtLocation` (`self.Sound`) _returnvalue (struct) 0.15 1.0 0.0 null null null)
                  (set `/Game/CyberSiege/Core/Animations/Characters/AI/ABP_MechEnemy.MechEnum` "NewEnumerator3" _asabp_mech_enemy)
                  (if (== (`GameplayStatics.GetObjectClass` (`BlackboardComponent.GetValueAsObject` _blackboard _bbcurrenttargetkeyname)) "/Game/CyberSiege/Core/Actors/Stationary/BP_Castle.BP_Castle_C")
                    ;[1 1 1] Attack Castle
                    (bind _outhit_2 (`KismetSystemLibrary.LineTraceSingleForObjects` _returnvalue (`BlackboardComponent.GetValueAsVector` (`self.Blackboard`) (`self.BBCastleLocationKeyName`)) _object_types))
                    (if (< (`.Distance` (`GameplayStatics.BreakHitResult` _outhit_2)) 500.0)
                      (if true
                        (`GameplayStatics.ApplyDamage` (`self.Castle`) (`self.BaseDamageMech`) (`AIBlueprintHelperLibrary.GetAIController` self) self)
                        (`KismetSystemLibrary.Delay` 1.4 :!label _label_2)
                        (set `self.CanDoDamage` true)
                        (set `/Game/CyberSiege/Core/Animations/Characters/AI/ABP_MechEnemy.MechEnum` "NewEnumerator0" _asabp_mech_enemy))
                      (else
                        (goto _label_2)))
                    (else
                      ;[1 1 1] Normal attack
                      (bind _outhit_3 (`KismetSystemLibrary.LineTraceSingleForObjects` :`Start` _returnvalue :`End` (`BlackboardComponent.GetLocationFromEntry` _blackboard _bbcurrenttargetkeyname) :`ObjectTypes` _object_types :`DrawTime` 2.0))
                      (bind (_bblockinghit _binitialoverlap _time _distance _location _impactpoint _normal _impactnormal _physmat _hitactor) (`GameplayStatics.BreakHitResult` _outhit_3))
                      (if (< _distance 500.0)
                        (if (not (`KismetMathLibrary.ClassIsChildOf` (`GameplayStatics.GetObjectClass` _hitactor) "/Game/CyberSiege/Core/Actors/Characters/AI/BP_BaseEnemy1.BP_BaseEnemy1_C"))
                          (`GameplayStatics.ApplyDamage` _hitactor (`self.BaseDamageMech`) (`AIBlueprintHelperLibrary.GetAIController` self) self)
                          (goto _label_2)
                          (else
                            (goto _label_2)))
                        (else
                          (goto _label_2))))))
                (:`CastFailed`
                  (`KismetSystemLibrary.PrintString` "Cast to AI shotgun failed (MechEnemy)")))))
          (else
            (goto _label))))
      (:`CastFailed`
        (`KismetSystemLibrary.PrintString` "not ABP_MechEnemy (Attack BP_MechEnemy)")))))

(event `self.Die`
  (params (HealthRatio :type "Float (single-precision)"))
  (bind _charactermovement (`self.CharacterMovement`))
  (bind _mapmarker (`self.MapMarker`))
  (set `self.IsDead` true)
  (bind _asabp_mech_enemy (cast `/Game/CyberSiege/Core/Animations/Characters/AI/ABP_MechEnemy` (`SkeletalMeshComponent.GetAnimInstance` (`self.Mesh`)))
    (:`then`
      (set `/Game/CyberSiege/Core/Animations/Characters/AI/ABP_MechEnemy.MechEnum` "NewEnumerator2" _asabp_mech_enemy)
      (`MovementComponent.StopMovementImmediately` _charactermovement)
      (`CharacterMovementComponent.DisableMovement` _charactermovement)
      (`Controller.UnPossess` (`AIBlueprintHelperLibrary.GetAIController` self))
      (`self.SetActorEnableCollision` false)
      (bind _returnvalue (`|SpawnActorFromClass` "/Game/CyberSiege/Core/Actors/Spawners/BP_ScrapSpawner.BP_ScrapSpawner_C" (`self.GetTransform` self) "AdjustIfPossibleButAlwaysSpawn" "OverrideRootScale" self null))
      (bind _output_get (set `self.ScrapSpawner` _returnvalue))
      (`BaseScrap.SetScrapAmount` _output_get 150.0)
      (`self.K2_AttachToActor` _output_get self "ScrapSpawnerSocket" "SnapToTarget" "KeepWorld" "KeepWorld" true)
      (`self.OnEnemyDied`)
      ;[1 1 1] temp
      (`/Game/CyberSiege/Core/Engine/BP_GameInstance.AddScore` (cast `/Game/CyberSiege/Core/Engine/BP_GameInstance` (`GameplayStatics.GetGameInstance`) :!pure true) self "NewEnumerator3")
      (`KismetMathLibrary.LinearColor_Set` (`/Game/CyberSiege/Core/Widgets/Minimap/BP_MapMarkerComponent.MarkerColor` _mapmarker) (struct :`A` 0.5))
      (`/Game/CyberSiege/Core/Widgets/Minimap/BP_MapMarkerComponent.UpdateMarkerProperties` _mapmarker)
      (`KismetSystemLibrary.Delay` (`self.TimeUntilDestroy`))
      (`self.K2_DestroyActor`)
      (if (!= (`self.ScrapSpawner`) null)
        (`self.K2_DestroyActor` (`self.ScrapSpawner`))))
    (:`CastFailed`
      (`KismetSystemLibrary.PrintString` "not ABP_MechEnemy (BP_MechEnemy)"))))

(event `self.StompBox.OnComponentBeginOverlap`
  (params (OverlappedComponent :type "PrimitiveComponent Object Reference") (OtherActor :type "Actor Object Reference") (OtherComp :type "PrimitiveComponent Object Reference") (OtherBodyIndex :type Integer) (bFromSweep :type Boolean) (SweepResult :type "HitResult Structure (by ref)"))
  (if (not (`KismetMathLibrary.ClassIsChildOf` (`GameplayStatics.GetObjectClass` OtherActor) "/Game/CyberSiege/Core/Actors/Characters/AI/BP_BaseEnemy1.BP_BaseEnemy1_C"))
    (`KismetArrayLibrary.Array_AddUnique` (`self.ActorsInStompBox`) OtherActor)))

(event `self.StompBox.OnComponentEndOverlap`
  (params (OverlappedComponent :type "PrimitiveComponent Object Reference") (OtherActor :type "Actor Object Reference") (OtherComp :type "PrimitiveComponent Object Reference") (OtherBodyIndex :type Integer))
  (`KismetArrayLibrary.Array_RemoveItem` (`self.ActorsInStompBox`) OtherActor))

(event `self.StompBox.OnComponentHit`
  (params (HitComponent :type "PrimitiveComponent Object Reference") (OtherActor :type "Actor Object Reference") (OtherComp :type "PrimitiveComponent Object Reference") (NormalImpulse :type "Vector Structure") (Hit :type "HitResult Structure (by ref)"))
  (`KismetSystemLibrary.PrintString` (`KismetSystemLibrary.GetDisplayName` OtherActor)))

(fn `GetLHSLocation`
  (returns (LeftHandSocket :type "Vector Structure"))
  (bind _childactorcomponent (`self.ChildActorComponent`))
  (if (== (`GameplayStatics.GetObjectClass` self) "BP_MechEnemy_C")
    (if (!= _childactorcomponent null)
      (bind _asbp_aishotgun (cast `/Game/CyberSiege/Core/Actors/Weapons/AI/BP_AIShotgun` (`ChildActorComponent.ChildActor` _childactorcomponent))
        (:`then`
          (return (`SceneComponent.GetSocketLocation` (`/Game/CyberSiege/Core/Actors/Weapons/BP_BaseWeapon.Mesh` _asbp_aishotgun) "LeftHandSocket")))
        (:`CastFailed`
          (`KismetSystemLibrary.PrintString` "Failed to cast to BP_AIShotgun (BP_MechEnemy)"))))))

(fn `GetPoints`
  (returns (Points :type "Float (double-precision)"))
  (return (* (`parent.GetPoints`) 2.0)))

(fn `UserConstructionScript`
  (`parent.UserConstructionScript`))