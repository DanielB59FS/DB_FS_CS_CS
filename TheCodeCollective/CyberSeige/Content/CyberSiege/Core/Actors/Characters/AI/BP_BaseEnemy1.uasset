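; Base enemy AI character that attacks the castle, player and defenses, with health scaled by wave in wave mode.
; Pawn sensing and AI perception write blackboard targets, using enemy counts to cap attackers per turret or blockade.
; Attacks briefly enable socketed hand collisions that deal damage on overlap, and pause-menu events toggle damage, movement and targeting.
; Death drops a health pickup or scrap, awards score, frees the turret slot and destroys the actor after a delay.
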(event `Die`
  (params (HealthRatio :type "Float (double-precision)"))
  (bind (_returnvalue_location _returnvalue_rotation) (`KismetMathLibrary.BreakTransform` (`self.GetTransform`)))
  (bind _charactermovement (`self.CharacterMovement`))
  (bind _mapmarker (`self.MapMarker`))
  (bind _returnvalue (`BlackboardComponent.GetValueAsObject` (`self.Blackboard`) (`self.BBTurretKeyName`)))
  (set `self.IsDead` true)
  (bind _asabp_base_enemy (cast `/Game/CyberSiege/Core/Animations/Characters/AI/ABP_BaseEnemy` (`SkeletalMeshComponent.GetAnimInstance` (`self.Mesh`)))
    (:`then`
      ;[0 0 0] Death
      (set `/Game/CyberSiege/Core/Animations/Characters/AI/ABP_BaseEnemy.EEnemyAIAnim` "NewEnumerator2" _asabp_base_enemy)
      (`MovementComponent.StopMovementImmediately` _charactermovement)
      (`CharacterMovementComponent.DisableMovement` _charactermovement)
      (`Controller.UnPossess` (`AIBlueprintHelperLibrary.GetAIController` self))
      (`self.SetActorEnableCollision` false)
      (if (>= (`KismetMathLibrary.RandomInteger` (`self.RandomMax`)) 95)
        (bind _returnvalue_2 (`|SpawnActorFromClass` "/Game/CyberSiege/Core/Actors/BP_HealthPickup.BP_HealthPickup_C" (`KismetMathLibrary.MakeTransform` _returnvalue_location _returnvalue_rotation (2.0 2.0 2.0)) "AlwaysSpawn" "OverrideRootScale" self null))
        (bind _output_get (set `self.HealthPickup` _returnvalue_2))
        (`self.K2_AttachToActor` _output_get self "HealthPickupSocket" "KeepWorld" "KeepWorld" "KeepRelative" false)
        (else
          (bind _returnvalue_3 (`|SpawnActorFromClass` "/Game/CyberSiege/Core/Actors/Spawners/BP_ScrapSpawner.BP_ScrapSpawner_C" (`self.GetTransform` self) "AdjustIfPossibleButAlwaysSpawn" "OverrideRootScale" self null))
          (bind _output_get_2 (set `self.ScrapSpawner` _returnvalue_3))
          (`BaseScrap.SetScrapAmount` _output_get_2 25.0)
          (`self.K2_AttachToActor` _output_get_2 self "ScrapSpawnerSocket" "SnapToTarget" "KeepWorld" "KeepWorld" true)))
      (`self.OnEnemyDied`)
      ;[1 1 1] temp
      (`/Game/CyberSiege/Core/Engine/BP_GameInstance.AddScore` (cast `/Game/CyberSiege/Core/Engine/BP_GameInstance` (`GameplayStatics.GetGameInstance`) :!pure true) self "NewEnumerator3")
      ;[1 1 1] Temporary, dead enemy marker
      (`KismetMathLibrary.LinearColor_Set` (`/Game/CyberSiege/Core/Widgets/Minimap/BP_MapMarkerComponent.MarkerColor` _mapmarker) (struct :`A` 0.5))
      (`/Game/CyberSiege/Core/Widgets/Minimap/BP_MapMarkerComponent.UpdateMarkerProperties` _mapmarker)
      (if (!= _returnvalue null)
        (message `/Game/CyberSiege/Core/Interfaces/BPI_Enemies.DecrementEnemyCount` _returnvalue))
      (`KismetSystemLibrary.Delay` (`self.TimeUntilDestroy`))
      (`self.K2_DestroyActor`)
      (if (!= (`self.ScrapSpawner`) null)
        (`self.K2_DestroyActor` (`self.ScrapSpawner`))
        (elif (!= (`self.HealthPickup`) null)
          (`self.K2_DestroyActor` (`self.HealthPickup`)))))
    (:`CastFailed`
      (`KismetSystemLibrary.PrintString` "not ABP_BaseEnemy (BP_BaseEnemy)"))))

(event `self.ReceiveBeginPlay`
  (bind _returnvalue (`GameplayStatics.GetGameMode`))
  (bind _healthcomponent (`self.HealthComponent`))
  (add `EffectComponent.OnShockEnded` (`self.Effect`) (`|CreateDelegate` (`self.HealthComponent`) :!event `On Shock Effect Ended`))
  (add `/Game/CyberSiege/Core/Actors/ActorComponents/BP_HealthComponent.OnDeath` (`self.HealthComponent`) (`|CreateDelegate` :!event `Die`))
  (set `self.GameMode` _returnvalue)
  (if (== (`GameplayStatics.GetObjectClass` _returnvalue) "/Game/CyberSiege/Core/GameModes/BP_WaveGameMode.BP_WaveGameMode_C")
    (bind _asbp_wave_game_mode (cast `/Game/CyberSiege/Core/GameModes/BP_WaveGameMode` _returnvalue))
    (add `/Game/CyberSiege/Core/GameModes/BP_WaveGameMode.OnRoundEnded` _asbp_wave_game_mode (`|CreateDelegate` :!event `IncreaseHealth`)))
  (add `self.OnEnemySpawned` (`|CreateDelegate` _asbp_wave_game_mode :!event `Enemy Added`))
  (add `self.OnEnemyDied` (`|CreateDelegate` _asbp_wave_game_mode :!event `Enemy Died`))
  (`self.OnEnemySpawned`)
  (set `self.Blackboard` (`AIBlueprintHelperLibrary.GetBlackboard` (`AIBlueprintHelperLibrary.GetAIController` self)))
  (bind _outactors (`GameplayStatics.GetAllActorsOfClass` "/Game/CyberSiege/Core/Actors/Stationary/BP_Castle.BP_Castle_C"))
  (bind _output_get (set `self.Castle` (`|GetArrayItem` _outactors)))
  (`BlackboardComponent.SetValueAsObject` (`self.Blackboard`) (`self.BBCastleKeyName`) _output_get)
  (bind _foundwidgets (`WidgetBlueprintLibrary.GetAllWidgetsOfClass` "/Game/CyberSiege/Core/Widgets/WBP_PauseMenu.WBP_PauseMenu_C"))
  (bind _output_get_2 (set `self.WBP_PauseMenu` (`|GetArrayItem` _foundwidgets)))
  (if (!= (`self.WBP_PauseMenu`) null)
    (add `/Game/CyberSiege/Core/Widgets/WBP_PauseMenu.OnEnemyDoDamageClick` _output_get_2 (`|CreateDelegate` :!event `EnemiesDoDamage`))
    (add `/Game/CyberSiege/Core/Widgets/WBP_PauseMenu.OnEnemiesMoveClick` _output_get_2 (`|CreateDelegate` :!event `EnemiesMove`))
    (add `/Game/CyberSiege/Core/Widgets/WBP_PauseMenu.OnEnemiesMoveTowardPlayerClick` _output_get_2 (`|CreateDelegate` :!event `EnemiesMoveTowardPlayer`))
    (add `/Game/CyberSiege/Core/Widgets/WBP_PauseMenu.OnEnemiesMoveTowardCastleClick` _output_get_2 (`|CreateDelegate` :!event `EnemiesMoveTowardCastle`)))
  (`PrimitiveComponent.SetCollisionEnabled` (`self.LeftHandCollision`) "NoCollision")
  (`PrimitiveComponent.SetCollisionEnabled` (`self.RightHandCollision`) "NoCollision")
  (bind _output_get_3 (set `/Game/CyberSiege/Core/Actors/ActorComponents/BP_HealthComponent.MaxHealth` (* (+ (/ (`KismetMathLibrary.Conv_IntToDouble` (`/Game/CyberSiege/Core/GameModes/BP_WaveGameMode.WaveCount` _asbp_wave_game_mode)) 10.0) 1.0) (`/Game/CyberSiege/Core/Actors/ActorComponents/BP_HealthComponent.MaxHealth` _healthcomponent)) _healthcomponent))
  (set `/Game/CyberSiege/Core/Actors/ActorComponents/BP_HealthComponent.CurrentHealth` _output_get_3 _healthcomponent))

(event `self.ReceiveTick`
  (params (DeltaSeconds :type "Float (single-precision)"))
  (`self.UpdateAnimations`)
  (`self.UpdateHealthBar`))

(event `self.PawnSensing.OnSeePawn`
  (params (Pawn :type "Pawn Object Reference"))
  ;[1 1 1] Has seen player
  (set `self.CanSeePlayer` true)
  (`BlackboardComponent.SetValueAsObject` (`self.Blackboard`) (`self.BBPlayerKeyName`) Pawn)
  (`KismetSystemLibrary.Delay` 5.0)
  (`BlackboardComponent.SetValueAsObject` (`self.Blackboard`) (`self.BBPlayerKeyName`) null))

(event `self.LeftHandCollision.OnComponentBeginOverlap`
  (params (OverlappedComponent :type "PrimitiveComponent Object Reference") (OtherActor :type "Actor Object Reference") (OtherComp :type "PrimitiveComponent Object Reference") (OtherBodyIndex :type Integer) (bFromSweep :type Boolean) (SweepResult :type "HitResult Structure (by ref)"))
  (bind _returnvalue (`self.GetOwner`))
  (bind _returnvalue_2 (`self.GetInstigatorController`))
  (bind _returnvalue_3 (`GameplayStatics.GetObjectClass` OtherActor))
  (bind _base_damage (`self.Base Damage`))
  (bind _sound (`self.Sound`))
  (bind _lefthandcollision (`self.LeftHandCollision`))
  ;[1 0 0] Damage what it is attacking with hands
  (for _array_element (`Actor.Tags` OtherActor)
    (if (and (!= OtherActor self) (!= _array_element "Enemy")) :!label _label
      (if (== _array_element "Castle")
        (`GameplayStatics.ApplyDamage` (`self.Castle`) _base_damage _returnvalue_2 _returnvalue)
        (else
          (`GameplayStatics.ApplyDamage` OtherActor _base_damage _returnvalue_2 _returnvalue)))
      (if (and (!= _returnvalue_3 "/Game/CyberSiege/Core/Actors/Characters/BP_BasePlayer.BP_BasePlayer_C") (!= _returnvalue_3 "/Game/CyberSiege/Core/Actors/Spawners/BP_ScrapSpawner.BP_ScrapSpawner_C"))
        (bind _hitlocation (`PrimitiveComponent.K2_LineTraceComponent` _lefthandcollision (`SceneComponent.K2_GetComponentLocation` _lefthandcollision) (`self.K2_GetActorLocation` OtherActor) true false false))
        (`GameplayStatics.SpawnEmitterAtLocation` "/Game/AssetMigration/MilitaryWeapSilver/FX/P_Impact_Metal_Medium_01.P_Impact_Metal_Medium_01" _hitlocation)
        (if (`self.CanPlaySound`)
          (set `self.CanPlaySound` false)
          (`GameplayStatics.PlaySoundAtLocation` _sound _hitlocation (struct) 0.15 1.0 0.0 null null null)
          (if (!= _sound null)
            (`KismetSystemLibrary.Delay` (/ (`SoundBase.Duration` _sound) 2.0))
            (set `self.CanPlaySound` true))))))
  (goto _label))

(event `self.RightHandCollision.OnComponentBeginOverlap`
  (params (OverlappedComponent :type "PrimitiveComponent Object Reference") (OtherActor :type "Actor Object Reference") (OtherComp :type "PrimitiveComponent Object Reference") (OtherBodyIndex :type Integer) (bFromSweep :type Boolean) (SweepResult :type "HitResult Structure (by ref)"))
  (bind _returnvalue (`self.GetOwner`))
  (bind _returnvalue_2 (`self.GetInstigatorController`))
  (bind _returnvalue_3 (`GameplayStatics.GetObjectClass` OtherActor))
  (bind _base_damage (`self.Base Damage`))
  (bind _righthandcollision (`self.RightHandCollision`))
  (bind _sound (`self.Sound`))
  ;[1 0 0] Damage what it is attacking with hands
  (for _array_element (`Actor.Tags` OtherActor)
    (if (and (!= OtherActor self) (!= _array_element "Enemy")) :!label _label_2
      (if (== _array_element "Castle")
        (`GameplayStatics.ApplyDamage` (`self.Castle`) _base_damage _returnvalue_2 _returnvalue)
        (else
          (`GameplayStatics.ApplyDamage` OtherActor _base_damage _returnvalue_2 _returnvalue)))
      (if (and (!= _returnvalue_3 "/Game/CyberSiege/Core/Actors/Characters/BP_BasePlayer.BP_BasePlayer_C") (!= _returnvalue_3 "/Game/CyberSiege/Core/Actors/Spawners/BP_ScrapSpawner.BP_ScrapSpawner_C"))
        (bind _hitlocation (`PrimitiveComponent.K2_LineTraceComponent` _righthandcollision (`SceneComponent.K2_GetComponentLocation` _righthandcollision) (`self.K2_GetActorLocation` OtherActor) true false false))
        (`GameplayStatics.SpawnEmitterAtLocation` "/Game/AssetMigration/MilitaryWeapSilver/FX/P_Impact_Metal_Medium_01.P_Impact_Metal_Medium_01" _hitlocation)
        (if (`self.CanPlaySound`)
          (set `self.CanPlaySound` false)
          (`GameplayStatics.PlaySoundAtLocation` _sound _hitlocation (struct) 0.15 1.0 0.0 null null null)
          (if (!= _sound null)
            (`KismetSystemLibrary.Delay` (/ (`SoundBase.Duration` _sound) 2.0))
            (set `self.CanPlaySound` true))))))
  (goto _label_2))

(event `self.AllEnemiesDead`
  (`BlackboardComponent.SetValueAsObject` (`self.Blackboard`) (`self.BBPlayerKeyName`) null))

(event `self.Attack`
  (params (ControlledPawn :type "Object Object Reference"))
  (`PrimitiveComponent.SetCollisionEnabled` (`self.LeftHandCollision`) "QueryOnly")
  (`PrimitiveComponent.SetCollisionEnabled` (`self.RightHandCollision`) "QueryOnly")
  (bind _asabp_base_enemy (cast `/Game/CyberSiege/Core/Animations/Characters/AI/ABP_BaseEnemy` (`SkeletalMeshComponent.GetAnimInstance` (`self.Mesh`)))
    (:`then`
      (set `/Game/CyberSiege/Core/Animations/Characters/AI/ABP_BaseEnemy.EEnemyAIAnim` "NewEnumerator3" _asabp_base_enemy)
      (`KismetSystemLibrary.Delay` 2.0)
      (set `/Game/CyberSiege/Core/Animations/Characters/AI/ABP_BaseEnemy.EEnemyAIAnim` "NewEnumerator0" _asabp_base_enemy)
      (`PrimitiveComponent.SetCollisionEnabled` (`self.LeftHandCollision`) "NoCollision")
      (`PrimitiveComponent.SetCollisionEnabled` (`self.RightHandCollision`) "NoCollision"))
    (:`CastFailed`
      (`KismetSystemLibrary.PrintString` "not ABP_BaseEnemy (BaseEnemy)"))))

(event `self.UpdateAnimations`
  (bind _returnvalue (`self.GetVelocity`))
  ;[1 1 0] Animations
  (bind _asabp_base_enemy (cast `/Game/CyberSiege/Core/Animations/Characters/AI/ABP_BaseEnemy` (`SkeletalMeshComponent.GetAnimInstance` (`self.Mesh`)))
    (:`then`
      (set `/Game/CyberSiege/Core/Animations/Characters/AI/ABP_BaseEnemy.Speed` (`KismetMathLibrary.VSize` _returnvalue) _asabp_base_enemy)
      (set `/Game/CyberSiege/Core/Animations/Characters/AI/ABP_BaseEnemy.Direction` (`AnimInstance.CalculateDirection` _asabp_base_enemy _returnvalue (`self.K2_GetActorRotation`)) _asabp_base_enemy))
    (:`CastFailed`
      (`KismetSystemLibrary.PrintString` "Could not cast anim instance to ABP_BaseEnemy (BP_BaseEnemy1)"))))

(event `self.AIPerception.OnTargetPerceptionUpdated`
  (params (Actor :type "Actor Object Reference") (Stimulus :type "AIStimulus Structure"))
  (bind _returnvalue (`GameplayStatics.GetObjectClass` Actor))
  (bind _returnvalue_2 (`GameplayStatics.GetObjectClass` Actor))
  (bind _blackboard (`self.Blackboard`))
  (bind _bbblockadekeyname (`self.BBBlockadeKeyName`))
  (if (not (`KismetMathLibrary.ClassIsChildOf` _returnvalue "/Game/CyberSiege/Core/Actors/Characters/BP_BaseCharacter.BP_BaseCharacter_C"))
    (if (== _returnvalue "/Game/CyberSiege/Core/Actors/Defenses/BP_Decoy.BP_Decoy_C")
      (`BlackboardComponent.SetValueAsObject` (`self.Blackboard`) (`self.BBDecoyKeyName`) Actor)
      (elif (== (`BlackboardComponent.GetValueAsObject` (`self.Blackboard`) (`self.BBTurretKeyName`)) null)
        (if (or (== _returnvalue_2 "/Game/CyberSiege/Core/Actors/Defenses/BP_BaseTurret.BP_BaseTurret_C") (== _returnvalue_2 "/Game/CyberSiege/Core/Actors/Defenses/BP_GrenadeTurret.BP_GrenadeTurret_C") (== _returnvalue_2 "/Game/CyberSiege/Core/Actors/Defenses/BP_SniperTurret.BP_SniperTurret_C"))
          (bind _enemycount (message `/Game/CyberSiege/Core/Interfaces/BPI_Enemies.GetEnemyCount` Actor))
          (if (< _enemycount 4)
            (`BlackboardComponent.SetValueAsObject` (`self.Blackboard`) (`self.BBTurretKeyName`) Actor)
            (message `/Game/CyberSiege/Core/Interfaces/BPI_Enemies.IncrementEnemyCount` Actor))
          (elif (== (`GameplayStatics.GetObjectClass` Actor) "/Game/CyberSiege/Core/Actors/Defenses/BP_Blockade.BP_Blockade_C")
            (bind _enemycount_2 (message `/Game/CyberSiege/Core/Interfaces/BPI_Enemies.GetEnemyCount` Actor))
            (if (< _enemycount_2 3)
              (if (== (`BlackboardComponent.GetValueAsObject` _blackboard _bbblockadekeyname) null)
                (`BlackboardComponent.SetValueAsObject` _blackboard _bbblockadekeyname Actor)
                (message `/Game/CyberSiege/Core/Interfaces/BPI_Enemies.IncrementEnemyCount` Actor)))))))))

(event `IncreaseHealth`
  (bind _healthcomponent (`self.HealthComponent`))
  (bind _gamemode (`self.GameMode`))
  (if (== (`GameplayStatics.GetObjectClass` _gamemode) "/Game/CyberSiege/Core/GameModes/BP_WaveGameMode.BP_WaveGameMode_C")
    (bind _asbp_wave_game_mode (cast `/Game/CyberSiege/Core/GameModes/BP_WaveGameMode` _gamemode))
    (if (<= (`/Game/CyberSiege/Core/GameModes/BP_WaveGameMode.WaveCount` _asbp_wave_game_mode) 20)
      (set `/Game/CyberSiege/Core/Actors/ActorComponents/BP_HealthComponent.MaxHealth` (* (`/Game/CyberSiege/Core/Actors/ActorComponents/BP_HealthComponent.MaxHealth` _healthcomponent) 1.1) _healthcomponent))))

(fn `EnemiesDoDamage`
  (params (EnemiesDoDamage :type Boolean))
  (if EnemiesDoDamage
    (set `self.Base Damage` 10.0)
    (else
      (set `self.Base Damage` 0.0))))

(fn `EnemiesMove`
  (params (EnemiesMove :type Boolean))
  (if EnemiesMove
    (`ActorComponent.Activate` (`self.CharacterMovement`) false)
    (else
      (`ActorComponent.Deactivate` (`self.CharacterMovement`)))))

(fn `EnemiesMoveTowardCastle`
  (if (not (`self.IsDead`))
    (`PawnSensingComponent.SetSensingUpdatesEnabled` (`self.PawnSensing`) false)
    (`BlackboardComponent.SetValueAsObject` (`self.Blackboard`) (`self.BBPlayerKeyName`) null)))

(fn `EnemiesMoveTowardPlayer`
  (`BlackboardComponent.SetValueAsObject` (`self.Blackboard`) (`self.BBPlayerKeyName`) (`GameplayStatics.GetPlayerPawn` 0)))

(fn `FindNewTurret`
  (params (CurrentTurret :type "Object Object Reference"))
  (bind _outactors (`GameplayStatics.GetAllActorsOfClass` "/Game/CyberSiege/Core/Actors/Defenses/BP_BaseTurret.BP_BaseTurret_C"))
  (for _array_element _outactors
    (if (!= CurrentTurret _array_element)
      (bind _enemycount (`self.GetEnemyCount` _array_element))
      (if (and (< _enemycount 4) (< (`self.GetDistanceTo` self _array_element) (`self.DistanceToTurret`)))
        (`BlackboardComponent.SetValueAsObject` (`self.Blackboard`) (`self.BBTurretKeyName`) _array_element)
        (`/Engine/EditorBlueprintResources/StandardMacros.IncrementInt` (`/Game/CyberSiege/Core/Actors/Defenses/BP_BaseTurret.EnemyCount` _array_element)))))
  (set `self.DistanceToTurret` 3.4028234663852886e+38))

(fn `GetEnemyCount`
  (returns (EnemyCount :type Integer))
  (return 0))

(fn `GetLHSLocation`
  (returns (LeftHandSocket :type "Vector Structure"))
  (return (0.0 0.0 0.0)))

(fn `GetPoints`
  (returns (Points :type "Float (double-precision)"))
  (return 5.0))

(fn `IsEnemy`
  (returns (Boolean :type Boolean))
  (return true))

(fn `UpdateHealthBar`
  (bind _healthbarwidget (`self.HealthBarWidget`))
  (bind _healthcomponent (`self.HealthComponent`))
  (bind _returnvalue (`WidgetComponent.GetWidget` (`self.HealthBarWidget`)))
  (if (not (`self.IsDead`))
    (bind _aswbp_health_bar (cast `/Game/CyberSiege/Core/Widgets/WBP_HealthBar` _returnvalue))
    (`ProgressBar.SetPercent` (`/Game/CyberSiege/Core/Widgets/WBP_HealthBar.HealthBar` _aswbp_health_bar) (`KismetMathLibrary.FClamp` (/ (`/Game/CyberSiege/Core/Actors/ActorComponents/BP_HealthComponent.CurrentHealth` _healthcomponent) (`/Game/CyberSiege/Core/Actors/ActorComponents/BP_HealthComponent.MaxHealth` _healthcomponent))))
    (if (`/Game/CyberSiege/Core/Actors/ActorComponents/BP_HealthComponent.IsShocked` (`self.HealthComponent`))
      (bind _effectbar (`/Game/CyberSiege/Core/Widgets/WBP_HealthBar.EffectBar` _aswbp_health_bar))
      (`Border.SetBrushColor` _effectbar (struct :`R` 0.048421 :`G` 0.153952 :`B` 0.619792 :`A` 1.0))
      (else
        (`Border.SetBrushColor` _effectbar (struct :`R` 1.0 :`G` 1.0 :`B` 1.0 :`A` 1.0))))
    (`SceneComponent.K2_SetWorldRotation` _healthbarwidget (`KismetMathLibrary.FindLookAtRotation` (`SceneComponent.K2_GetComponentLocation` _healthbarwidget) (`SceneComponent.K2_GetComponentLocation` (`PlayerCameraManager.TransformComponent` (`GameplayStatics.GetPlayerCameraManager` 0)))) false false)
    (else
      (`Widget.SetVisibility` _returnvalue "Hidden"))))

(fn `UserConstructionScript`
  (`parent.UserConstructionScript`)
  (`SceneComponent.K2_AttachToComponent` (`self.LeftHandCollision`) (`self.Mesh`) "Hand_L" "KeepRelative" "KeepRelative" "KeepRelative" true)
  (`SceneComponent.K2_AttachToComponent` (`self.RightHandCollision`) (`self.Mesh`) "Hand_R" "KeepRelative" "KeepRelative" "KeepRelative" true)
  (`SceneComponent.K2_AttachToComponent` (`self.HeadCollision`) (`self.Mesh`) "head" "KeepRelative" "KeepRelative" "KeepRelative" true)
  (if (not (`self.bEnableHeadCollision`))
    (`PrimitiveComponent.SetCollisionEnabled` (`self.HeadCollision`) "NoCollision")))