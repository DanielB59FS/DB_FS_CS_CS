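; BP_ActivatorInstance is a quest actor that connects QuestActivator events to gameplay effects.
; On BeginPlay it binds wave timer start once the BP_WaveGameMode cast succeeds, and menu item unlock and scrap rewards once the BP_BasePlayer cast succeeds.
; It also binds the turret damage event; its DamageAllTurrets event applies fixed damage to every Turrets actor in the level.
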(event `Damage All Turrets`
  (bind _outactors (`GameplayStatics.GetAllActorsOfClass` "/Script/CyberSeige.Turrets"))
  (for _array_element _outactors
    (`GameplayStatics.ApplyDamage` _array_element 35.0)))

(event `self.ReceiveBeginPlay`
  (bind _questactivator (`self.QuestActivator`))
  (bind _asbp_wave_game_mode (cast `/Game/CyberSiege/Core/GameModes/BP_WaveGameMode` (`GameplayStatics.GetGameMode`))
    (:`then`
      (add `QuestActivatorComponent.OnStartWaveTimer` (`self.QuestActivator`) (`|CreateDelegate` _asbp_wave_game_mode :!event `Toggle Timer`)))
    (:`CastFailed`
      _))
  (bind _asbp_base_player (cast `/Game/CyberSiege/Core/Actors/Characters/BP_BasePlayer` (`GameplayStatics.GetPlayerPawn` 0))
    (:`then`
      (add `QuestActivatorComponent.OnEnableMenuItem` _questactivator (`|CreateDelegate` (`/Game/CyberSiege/Core/Actors/Characters/BP_BasePlayer.Get Build HUD` _asbp_base_player) :!event `EnableMenuItem`))
      (add `QuestActivatorComponent.OnGiveScrap` _questactivator (`|CreateDelegate` (`/Game/CyberSiege/Core/Actors/Characters/BP_BasePlayer.Build Component` _asbp_base_player) :!event `ChangeScrapCount`)))
    (:`CastFailed`
      _))
  (add `QuestActivatorComponent.OnDamageTurrets` _questactivator (`|CreateDelegate` :!event `Damage All Turrets`)))

(fn `UserConstructionScript`)