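; BP_QuestManager is the quest manager actor, running the active quest's setup and showing its dialogue and completion messages on the player's HUD.
; Shortly after BeginPlay, it binds activator components on the quest steps to wave-timer and menu-item events, using the wave game mode and player as cast checks.
; SetupQuest binds steps, configures trigger indicators and completion callbacks, then broadcasts the steps to the quest list.
; BindTrigger is an empty stub.
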(event `self.ReceiveBeginPlay`
  (bind (_questkey _questcompletemessage _queststeps) (break `Quest` (`self.ActiveQuest`)))
  (`KismetSystemLibrary.Delay` 5.0)
  (if (not (`KismetStringLibrary.EqualEqual_StrStr` _questkey "NULL"))
    (for _array_element _queststeps
      (for _array_element_2 (`.Activators` (break `QuestStep` _array_element))
        (bind _returnvalue (`self.GetComponentByClass` _array_element_2 "/Script/CyberSeige.QuestActivatorComponent"))
        (if (`KismetSystemLibrary.IsValid` _returnvalue)
          (bind _asbp_wave_game_mode (cast `/Game/CyberSiege/Core/GameModes/BP_WaveGameMode` (`GameplayStatics.GetGameMode`))
            (:`then`
              (add `QuestActivatorComponent.OnStartWaveTimer` _returnvalue (`|CreateDelegate` _asbp_wave_game_mode :!event `Toggle Timer`)))
            (:`CastFailed`
              _))
          (bind _asbp_base_player (cast `/Game/CyberSiege/Core/Actors/Characters/BP_BasePlayer` (`GameplayStatics.GetPlayerPawn` 0)))
          (add `QuestActivatorComponent.OnEnableMenuItem` _returnvalue (`|CreateDelegate` (`/Game/CyberSiege/Core/Actors/Characters/BP_BasePlayer.Get Build HUD` _asbp_base_player) :!event `EnableMenuItem`)))))))

(event `self.ReceiveSetHudMessage`
  (bind (_queststeptext _triggers _activators _binitialstep _bfinalstep _bskipifnotriggers _bismultitrigger _busesindicator _dialoguetext _boundtriggercount _triggersneeded _triggershit _stepnumber _dialogueboximage) (break `QuestStep` (`.ActiveStep` (break `Quest` (`self.ActiveQuest`)))))
  (bind _asbp_base_player (cast `/Game/CyberSiege/Core/Actors/Characters/BP_BasePlayer` (`GameplayStatics.GetPlayerPawn` 0)))
  (`/Game/CyberSiege/Core/Widgets/WBP_HUD.SetHUDMessage` (`/Game/CyberSiege/Core/Actors/Characters/BP_BasePlayer.Get Gameplay HUD` _asbp_base_player) _dialoguetext 5.0 true _dialogueboximage))

(event `self.ReceiveQuestFinished`
  (bind (_questkey _questcompletemessage _queststeps _activestep) (break `Quest` (`self.ActiveQuest`)))
  (bind _asbp_base_player (cast `/Game/CyberSiege/Core/Actors/Characters/BP_BasePlayer` (`GameplayStatics.GetPlayerPawn` 0)))
  (`/Game/CyberSiege/Core/Widgets/WBP_HUD.SetHUDMessage` (`/Game/CyberSiege/Core/Actors/Characters/BP_BasePlayer.Get Gameplay HUD` _asbp_base_player) (`KismetTextLibrary.Conv_TextToString` _questcompletemessage) 5.0 true (`.DialogueBoxImage` (break `QuestStep` _activestep)))
  (set `self.bQuestSetupComplete` false))

(event `self.ReceiveSetupQuest`
  (bind _activequest (`self.ActiveQuest`))
  (bind (_questkey _questcompletemessage _queststeps) (break `Quest` (`self.ActiveQuest`)))
  (bind (_questkey_2 _questcompletemessage_2 _queststeps_2) (break `Quest` _activequest))
  (for _array_element _queststeps_2
    (bind _returnvalue (`self.BindStep` _array_element))
    (`|VariableSetRef` _array_element _returnvalue)
    (bind (_queststeptext _triggers _activators _binitialstep _bfinalstep _bskipifnotriggers _bismultitrigger _busesindicator) (break `QuestStep` _array_element))
    (for _array_element_2 _triggers
      (bind _asbp_quest_trigger_component (cast `/Game/CyberSiege/Core/Actors/ActorComponents/BP_QuestTriggerComponent` _array_element_2))
      (set `/Game/CyberSiege/Core/Actors/ActorComponents/BP_QuestTriggerComponent.bUseIndicator` _busesindicator _asbp_quest_trigger_component)
      (add `/Game/CyberSiege/Core/Actors/ActorComponents/BP_QuestTriggerComponent.OnTriggerComplete` _asbp_quest_trigger_component (`|CreateDelegate` :!event `CompleteStep`)))
    (setmembers `QuestStep` :`StructRef` _array_element :`Triggers` _triggers))
  (setmembers `Quest` :`StructRef` _activequest :`QuestSteps` _queststeps_2)
  (`self.BindQuest`)
  (set `self.bQuestSetupComplete` true)
  (`self.OnSendInfoToQuestList` _questkey _queststeps))

(fn `BindTrigger`
  (params (Trigger :type "/Game/Sandboxes/Chadwick/BP_BlueprintQuestTrigger Object Reference") (BoundStep :type Integer)))

(fn `UserConstructionScript`)