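; BP_QuestGiver is an interactable actor that hands out one quest, keyed by QuestKey, once the wave count reaches WaveUnlock.
; Interact either shows a HUD refusal or sets GaveQuest, then StartQuest loads the quest into BP_QuestManager unless one is active.
; It binds to wave and quest manager events, with functions toggling map markers through color alpha.
; Custom depth rendering provides the outline.
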(event `self.ReceiveBeginPlay`
  (`KismetSystemLibrary.K2_SetTimerDelegate` (`|CreateDelegate` :!event `StopOutline`) 0.25 true)
  (bind _returnvalue (`GameplayStatics.GetActorOfClass` "/Game/CyberSiege/Core/Engine/BP_WaveManager.BP_WaveManager_C"))
  (add `WaveManager.OnWaveEnded` _returnvalue (`|CreateDelegate` :!event `Check Wave Count`))
  (bind _returnvalue_2 (`GameplayStatics.GetActorOfClass` "/Game/CyberSiege/Core/Actors/Quest/BP_QuestManager.BP_QuestManager_C"))
  (if (`KismetSystemLibrary.IsValid` _returnvalue_2)
    (add `QuestManager.OnQuestBegin` _returnvalue_2 (`|CreateDelegate` :!event `Disable All Quest Map Markers`))
    (add `QuestManager.OnQuestEnded` _returnvalue_2 (`|CreateDelegate` :!event `Enable All Quest Map Markers`))))

(event `/Game/CyberSiege/Core/Interfaces/BPI_Interact.Interact`
  (params (`Interacting Actor` :type "Actor Object Reference"))
  (bind _asbp_wave_game_mode (cast `/Game/CyberSiege/Core/GameModes/BP_WaveGameMode` (`GameplayStatics.GetGameMode`)))
  (if (or (`self.bGaveQuest`) (< (`/Game/CyberSiege/Core/GameModes/BP_WaveGameMode.WaveCount` _asbp_wave_game_mode) (`self.WaveUnlock`)))
    (bind _asbp_base_player (cast `/Game/CyberSiege/Core/Actors/Characters/BP_BasePlayer` (`GameplayStatics.GetPlayerPawn` 0)))
    (`/Game/CyberSiege/Core/Widgets/WBP_HUD.SetHUDMessage` (`/Game/CyberSiege/Core/Actors/Characters/BP_BasePlayer.Get Gameplay HUD` _asbp_base_player) "I don't have any tasks for you." 3.0 true (`self.QuestGiverIcon`))
    (else
      (set `self.bGaveQuest` true)
      (`self.Start Quest`))))

(event `/Game/CyberSiege/Core/Interfaces/BPI_Interact.StartOutline`
  (if (`KismetSystemLibrary.IsValid` (`self.StaticMesh`))
    (`PrimitiveComponent.SetRenderCustomDepth` (`self.StaticMesh`) true))
  (if (`KismetSystemLibrary.IsValid` (`self.SkeletalMesh`))
    (`PrimitiveComponent.SetRenderCustomDepth` (`self.SkeletalMesh`) true)))

(event `/Game/CyberSiege/Core/Interfaces/BPI_Interact.StopOutline`
  (if (`KismetSystemLibrary.IsValid` (`self.StaticMesh`))
    (`PrimitiveComponent.SetRenderCustomDepth` (`self.StaticMesh`) false))
  (if (`KismetSystemLibrary.IsValid` (`self.SkeletalMesh`))
    (`PrimitiveComponent.SetRenderCustomDepth` (`self.SkeletalMesh`) false)))

(event `Check Wave Count`
  (bind _asbp_wave_game_mode (cast `/Game/CyberSiege/Core/GameModes/BP_WaveGameMode` (`GameplayStatics.GetGameMode`)))
  (if (>= (`/Game/CyberSiege/Core/GameModes/BP_WaveGameMode.WaveCount` _asbp_wave_game_mode) (`self.WaveUnlock`))
    (`self.Enable Map Marker`)
    (else
      (`self.Disable Map Marker`))))

(event `Disable All Quest Map Markers`
  (bind _outactors (`GameplayStatics.GetAllActorsOfClass` "BP_QuestGiver_C"))
  (for _array_element _outactors
    (`self.Disable Map Marker` _array_element)))

(event `Enable All Quest Map Markers`
  (bind _outactors (`GameplayStatics.GetAllActorsOfClass` "BP_QuestGiver_C"))
  (for _array_element _outactors
    (`self.Check Wave Count` _array_element)))

(fn `Disable Map Marker`
  (bind _bp_mapmarkercomponent (`self.BP_MapMarkerComponent`))
  (bind _structout (setmembers `LinearColor` :`StructRef` (`/Game/CyberSiege/Core/Widgets/Minimap/BP_MapMarkerComponent.MarkerColor` (`self.BP_MapMarkerComponent`)) :`A` 0.0))
  (set `/Game/CyberSiege/Core/Widgets/Minimap/BP_MapMarkerComponent.MarkerColor` _structout _bp_mapmarkercomponent)
  (`/Game/CyberSiege/Core/Widgets/Minimap/BP_MapMarkerComponent.UpdateMarkerProperties` _bp_mapmarkercomponent))

(fn `Enable Map Marker`
  (bind _bp_mapmarkercomponent (`self.BP_MapMarkerComponent`))
  (if (not (`self.bGaveQuest`))
    (bind _structout (setmembers `LinearColor` :`StructRef` (`/Game/CyberSiege/Core/Widgets/Minimap/BP_MapMarkerComponent.MarkerColor` (`self.BP_MapMarkerComponent`)) :`A` 1.0))
    (set `/Game/CyberSiege/Core/Widgets/Minimap/BP_MapMarkerComponent.MarkerColor` _structout _bp_mapmarkercomponent)
    (`/Game/CyberSiege/Core/Widgets/Minimap/BP_MapMarkerComponent.UpdateMarkerProperties` _bp_mapmarkercomponent)))

(fn `Start Quest`
  (bind _returnvalue (`GameplayStatics.GetActorOfClass` "/Game/CyberSiege/Core/Actors/Quest/BP_QuestManager.BP_QuestManager_C"))
  (if (`KismetSystemLibrary.IsValid` _returnvalue)
    (if (`QuestManager.bQuestSetupComplete` _returnvalue)
      (bind _asbp_base_player (cast `/Game/CyberSiege/Core/Actors/Characters/BP_BasePlayer` (`GameplayStatics.GetPlayerPawn` 0)))
      (`/Game/CyberSiege/Core/Widgets/WBP_HUD.SetHUDMessage` (`/Game/CyberSiege/Core/Actors/Characters/BP_BasePlayer.Get Gameplay HUD` _asbp_base_player) "It looks like you already have a quest. Come back when you're finished" 4.0 true (`self.QuestGiverIcon`))
      (else
        (bind (_retrieved_quest _returned_valid_quest) (`/Game/CyberSiege/Core/Engine/BP_QuestLibraryComponent.GetQuest` (`/Game/CyberSiege/Core/Actors/Quest/BP_QuestManager.Quest Library` _returnvalue) (`self.QuestKey`)))
        (if _returned_valid_quest
          (set `QuestManager.ActiveQuest` _retrieved_quest _returnvalue)
          (`QuestManager.StartTimers` _returnvalue)
          (setmembers `SingleAnimationPlayData` :`StructRef` (`SkeletalMeshComponent.AnimationData` (`self.SkeletalMesh`)) :`AnimToPlay` "/Game/CyberSiege/Art/Cinematics/Tutorial/Animations/Breathing_Idle.Breathing_Idle")
          (`self.Disable Map Marker`)
          (`GameplayStatics.PlaySoundAtLocation` "/Game/CyberSiege/Audio/UI/A_Menu_Selection_Click_Cue.A_Menu_Selection_Click_Cue" (`self.K2_GetActorLocation`) (struct) 1.0 1.0 0.0 null null null)
          (else
            (`KismetSystemLibrary.PrintString` "Returned invalid quest")))))
    (else
      (`KismetSystemLibrary.PrintString` "Could not retrieve quest manager"))))

(fn `UserConstructionScript`)