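; BP_QuestIndicator is a quest marker actor whose Arrow component continuously bobs up and down.
; Each Tick advances a phase by delta time and a speed variable, resetting it to zero near two pi.
; The phase's cosine, scaled by a height multiplier, is added as a vertical world offset.
; That per-frame offset is not scaled by delta time, so bob height varies with frame rate.
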(event `self.ReceiveTick`
  (params (DeltaSeconds :type "Float (single-precision)"))
  (bind _returnvalue (+ (* DeltaSeconds (`self.FloatSpeed`)) (`self.FloatDelta`)))
  (if (>= _returnvalue 6.28)
    (set `self.FloatDelta` 0.0)
    (else
      (bind _output_get (set `self.FloatDelta` _returnvalue))))
  (`SceneComponent.K2_AddWorldOffset` (`self.Arrow`) (`KismetMathLibrary.MakeVector` 0.0 0.0 (* (`KismetMathLibrary.Cos` _output_get) (`self.FloatHeightMult`))) false false))

(fn `UserConstructionScript`)