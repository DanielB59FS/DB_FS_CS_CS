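; Quest trigger actor with a physics-capable static mesh that completes a quest step when a BP_BasePlayer overlaps its Box.
; On overlap, it calls CompleteStep and DisableTrigger on BPQuestTriggerComponent, then turns off box and mesh collision, stops mesh physics and hides the mesh instead of destroying the actor.
; A separate DisableTriggerOnDestroy event also disables the quest trigger component.
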(event `self.Box.OnComponentBeginOverlap`
  (params (OverlappedComponent :type "PrimitiveComponent Object Reference") (OtherActor :type "Actor Object Reference") (OtherComp :type "PrimitiveComponent Object Reference") (OtherBodyIndex :type Integer) (bFromSweep :type Boolean) (SweepResult :type "HitResult Structure (by ref)"))
  (bind _bp_questtriggercomponent (`self.BP_QuestTriggerComponent`))
  (bind _staticmesh (`self.StaticMesh`))
  (cast `/Game/CyberSiege/Core/Actors/Characters/BP_BasePlayer` OtherActor)
  (if (`KismetSystemLibrary.IsValid` _bp_questtriggercomponent)
    _
    (else
      _))
  (`/Game/CyberSiege/Core/Actors/ActorComponents/BP_QuestTriggerComponent.Complete Step` _bp_questtriggercomponent)
  (`/Game/CyberSiege/Core/Actors/ActorComponents/BP_QuestTriggerComponent.DisableTrigger` _bp_questtriggercomponent)
  (`PrimitiveComponent.SetCollisionEnabled` (`self.Box`) "NoCollision")
  (`PrimitiveComponent.SetSimulatePhysics` _staticmesh false)
  (`PrimitiveComponent.SetCollisionEnabled` _staticmesh "NoCollision")
  (`SceneComponent.SetVisibility` _staticmesh false true))

(event `Disable Trigger On Destroy`
  (params (DestroyedActor :type "Actor Object Reference"))
  (`/Game/CyberSiege/Core/Actors/ActorComponents/BP_QuestTriggerComponent.DisableTrigger` (`self.BP_QuestTriggerComponent`)))

(fn `UserConstructionScript`)