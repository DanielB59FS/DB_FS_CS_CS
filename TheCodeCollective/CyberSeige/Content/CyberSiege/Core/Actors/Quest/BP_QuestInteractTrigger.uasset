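; Interactable quest trigger actor that completes a quest step on its BPQuestTriggerComponent when interacted with.
; While the trigger is active, outline events toggle custom depth rendering on its static or skeletal mesh.
; It binds to the component's completion event at BeginPlay, with a wrapper event for clearing the outline.
; Outlining the skeletal mesh also starts a short one-shot timer.
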(event `self.ReceiveBeginPlay`
  (add `/Game/CyberSiege/Core/Actors/ActorComponents/BP_QuestTriggerComponent.OnTriggerComplete` (`self.BP_QuestTriggerComponent`) (`|CreateDelegate` :!event `Stop Outline With Args`)))

(event `self.Interact`
  (params (`Interacting Actor` :type "Actor Object Reference"))
  (`/Game/CyberSiege/Core/Actors/ActorComponents/BP_QuestTriggerComponent.Complete Step` (`self.BP_QuestTriggerComponent`)))

(event `self.StartOutline`
  (if (`/Game/CyberSiege/Core/Actors/ActorComponents/BP_QuestTriggerComponent.bTriggerActive` (`self.BP_QuestTriggerComponent`))
    (if (`KismetSystemLibrary.IsValid` (`self.StaticMesh`))
      (`PrimitiveComponent.SetRenderCustomDepth` (`self.StaticMesh`) true))
    (if (`KismetSystemLibrary.IsValid` (`self.SkeletalMesh`))
      (`PrimitiveComponent.SetRenderCustomDepth` (`self.SkeletalMesh`) true)
      (`KismetSystemLibrary.K2_SetTimerDelegate` (`|CreateDelegate` :!event `StopOutline`) 0.1))))

(event `self.StopOutline`
  (if (`/Game/CyberSiege/Core/Actors/ActorComponents/BP_QuestTriggerComponent.bTriggerActive` (`self.BP_QuestTriggerComponent`))
    (if (`KismetSystemLibrary.IsValid` (`self.StaticMesh`))
      (`PrimitiveComponent.SetRenderCustomDepth` (`self.StaticMesh`) false))
    (if (`KismetSystemLibrary.IsValid` (`self.SkeletalMesh`))
      (`PrimitiveComponent.SetRenderCustomDepth` (`self.SkeletalMesh`) false))))

(event `Stop Outline With Args`
  (params (Trigger :type "SceneComponent Object Reference"))
  (`self.StopOutline`))

(fn `UserConstructionScript`)