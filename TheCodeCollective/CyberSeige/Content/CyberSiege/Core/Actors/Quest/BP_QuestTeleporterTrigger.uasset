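; Quest trigger actor that completes teleporter-related quest steps when a Teleporter actor overlaps its box volume.
; On overlap it completes the step of the first active trigger, checking Teleporter1Trigger before Teleporter2Trigger, so only one step completes per overlap.
; GetBoundStep exposes only the step bound to Teleporter1Trigger.
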(event `self.Box.OnComponentBeginOverlap`
  (params (OverlappedComponent :type "PrimitiveComponent Object Reference") (OtherActor :type "Actor Object Reference") (OtherComp :type "PrimitiveComponent Object Reference") (OtherBodyIndex :type Integer) (bFromSweep :type Boolean) (SweepResult :type "HitResult Structure (by ref)"))
  (bind _teleporter1trigger (`self.Teleporter1Trigger`))
  (bind _teleporter2trigger (`self.Teleporter2Trigger`))
  (cast `Teleporter` OtherActor)
  (if (`/Game/CyberSiege/Core/Actors/ActorComponents/BP_QuestTriggerComponent.bTriggerActive` _teleporter1trigger)
    (`/Game/CyberSiege/Core/Actors/ActorComponents/BP_QuestTriggerComponent.Complete Step` _teleporter1trigger)
    (elif (`/Game/CyberSiege/Core/Actors/ActorComponents/BP_QuestTriggerComponent.bTriggerActive` _teleporter2trigger)
      (`/Game/CyberSiege/Core/Actors/ActorComponents/BP_QuestTriggerComponent.Complete Step` _teleporter2trigger))))

(fn `GetBoundStep`
  (returns (ReturnValue :type Integer))
  (return (`/Game/CyberSiege/Core/Actors/ActorComponents/BP_QuestTriggerComponent.BoundStep` (`self.Teleporter1Trigger`))))

(fn `UserConstructionScript`)