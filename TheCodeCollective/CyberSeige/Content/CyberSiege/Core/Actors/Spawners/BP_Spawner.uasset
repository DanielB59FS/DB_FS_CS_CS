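; Enemy spawner actor that spawns enemy classes passed to it through the CallSpawners event.
; Each class is appended to EnemyQueue, then SpawnEnemy immediately spawns the front entry at the actor's transform and removes it.
; Spawning adjusts for collisions but always succeeds in placement.
; The timer calls for delayed or looping spawns are unconnected, and GetLeftHandSocketTransform is an empty stub.
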(event `self.ReceiveBeginPlay`)

(event `/Game/CyberSiege/Core/Interfaces/BPI_Enemies.CallSpawners`
  (params (EnemyClass :type "/Game/CyberSiege/Core/Actors/Characters/BP_BaseCharacter Class Reference"))
  (`self.AddEnemyToQueue` EnemyClass))

(fn `AddEnemyToQueue`
  (params (EnemyClass :type "/Game/CyberSiege/Core/Actors/Characters/BP_BaseCharacter Class Reference (by ref)"))
  (`KismetArrayLibrary.Array_Add` (`self.EnemyQueue`) EnemyClass)
  (`self.SpawnEnemy`))

(fn `GetLeftHandSocketTransform`
  (returns (LeftHandSocket :type "Transform Structure"))
  (return))

(fn `SpawnEnemy`
  (returns (Success :type Boolean))
  (if (`KismetArrayLibrary.Array_IsValidIndex` (`self.EnemyQueue`))
    (`|SpawnActorFromClass` (`|GetArrayItem` (`self.EnemyQueue`)) (`self.GetTransform`) "AdjustIfPossibleButAlwaysSpawn" "OverrideRootScale" null null)
    (`KismetArrayLibrary.Array_Remove` (`self.EnemyQueue`))
    (return true)
    (else
      (return false))))

(fn `UserConstructionScript`)