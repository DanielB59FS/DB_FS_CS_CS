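; Player controller for the CyberSiege wave game that manages the pause menu, map toggle input and end-of-game flow.
; Pause toggling swaps input mode, cursor and HUD visibility, backing out of stacked menu panels before resuming.
; The wave game mode's GameEnded event locks the menu open with the result and updates GameInstance records, detecting wins by a temporary message substring check.
; Tick feeds unpaused play time to the GameInstance.
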(event `self.ReceiveBeginPlay`
  (`|ExecutionSequence`
    (:`then_0`
      (`WidgetBlueprintLibrary.SetInputMode_GameOnly` self))
    (:`then_1`
      (bind _returnvalue (`|CreateWidget` "/Game/CyberSiege/Core/Widgets/WBP_PauseMenu.WBP_PauseMenu_C" self))
      (bind _output_get (set `self.PauseMenu` _returnvalue))
      (`Widget.SetVisibility` _output_get "Hidden")
      (`UserWidget.AddToViewport` _output_get 0))
    (:`then_2`
      (bind _asbp_wave_game_mode (cast `/Game/CyberSiege/Core/GameModes/BP_WaveGameMode` (`GameplayStatics.GetGameMode`)))
      (add `/Game/CyberSiege/Core/GameModes/BP_WaveGameMode.GameEnded` _asbp_wave_game_mode (`|CreateDelegate` :!event `GameEnded`)))))

(event `UpdateHighScore`
  (`/Game/CyberSiege/Core/Engine/BP_GameInstance.CheckHighScore` (cast `/Game/CyberSiege/Core/Engine/BP_GameInstance` (`GameplayStatics.GetGameInstance`) :!pure true)))

(event `InputAction|Map`
  (params (Key :type "Key Structure"))
  (:`Pressed`
    (`/Game/CyberSiege/Core/Widgets/HUD/BP_HUD.ToggleMap` (cast `/Game/CyberSiege/Core/Widgets/HUD/BP_HUD` (`self.GetHUD`) :!pure true))))

(event `UpdateTimeRecord`
  (`/Game/CyberSiege/Core/Engine/BP_GameInstance.UpdateTimeRecord` (cast `/Game/CyberSiege/Core/Engine/BP_GameInstance` (`GameplayStatics.GetGameInstance`) :!pure true)))

(event `UpdateWaveRank`
  (`/Game/CyberSiege/Core/Engine/BP_GameInstance.CheckWaveRank` (cast `/Game/CyberSiege/Core/Engine/BP_GameInstance` (`GameplayStatics.GetGameInstance`) :!pure true) (`/Game/CyberSiege/Core/GameModes/BP_WaveGameMode.WaveCount` (cast `/Game/CyberSiege/Core/GameModes/BP_WaveGameMode` (`GameplayStatics.GetGameMode`) :!pure true))))

(event `InputAction|Pause` :paused true
  (params (Key :type "Key Structure"))
  (:`Pressed`
    (`self.TogglePauseMenu`)))

(event `GameEnded`
  (params (Message :type Text))
  (bind _returnvalue (`KismetTextLibrary.Conv_TextToString` Message))
  (`/Game/CyberSiege/Core/Widgets/WBP_PauseMenu.ResultState` (`self.PauseMenu`) Message)
  (set `self.bGameEnded` true)
  (bind _asbp_wave_game_mode (cast `/Game/CyberSiege/Core/GameModes/BP_WaveGameMode` (`GameplayStatics.GetGameMode`)))
  (remove `/Game/CyberSiege/Core/GameModes/BP_WaveGameMode.GameEnded` _asbp_wave_game_mode (`|CreateDelegate` :!event `GameEnded`))
  (`self.TogglePauseMenu`)
  (`self.UpdateWaveRank`)
  (`self.UpdateHighScore`)
  (if (or (`KismetStringLibrary.Contains` _returnvalue "win") (`KismetStringLibrary.Contains` _returnvalue "won"))
    (`self.UpdateTimeRecord`)))

(event `TogglePauseMenu`
  (bind _pausemenu (`self.PauseMenu`))
  (bind _pausemenu_2 (`self.PauseMenu`))
  (bind _ashudmanager (cast `HUDManager` (`self.GetHUD` self) :!pure true))
  (if (`|EnumEquality` (`Widget.GetVisibility` _pausemenu) "Hidden")
    (`Widget.SetVisibility` (`self.PauseMenu`) "Visible")
    (`WidgetBlueprintLibrary.SetInputMode_UIOnlyEx` self null "LockAlways")
    (set `self.bShowMouseCursor` true)
    (`GameplayStatics.SetGamePaused` true)
    (`HUDManager.SetVisibility` _ashudmanager "Hidden")
    (elif (> (`KismetArrayLibrary.Array_Length` (`/Game/CyberSiege/Core/Widgets/WBP_PauseMenu.PanelStack` _pausemenu)) 0)
      (`/Game/CyberSiege/Core/Widgets/WBP_TextButton.OnClick` (`/Game/CyberSiege/Core/Widgets/WBP_PauseMenu.ButtonBack` _pausemenu_2))
      (elif (not (`self.bGameEnded`))
        (`Widget.SetVisibility` _pausemenu_2 "Hidden")
        (set `self.bShowMouseCursor` false)
        (`WidgetBlueprintLibrary.SetInputMode_GameOnly` self)
        (`GameplayStatics.SetGamePaused` false)
        (`HUDManager.SetVisibility` _ashudmanager "Visible")))))

(event `self.ReceiveTick`
  (params (DeltaSeconds :type "Float (single-precision)"))
  (if (not (`GameplayStatics.IsGamePaused`))
    (`/Game/CyberSiege/Core/Engine/BP_GameInstance.UpdateDurations` (cast `/Game/CyberSiege/Core/Engine/BP_GameInstance` (`GameplayStatics.GetGameInstance`) :!pure true) DeltaSeconds)))

(fn `UserConstructionScript`)